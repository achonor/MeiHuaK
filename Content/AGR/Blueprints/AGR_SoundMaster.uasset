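; AGR_SoundMaster is a component handling footsteps, keyed speech, ambient sound and wind for its owning character.
; Footsteps, triggered by name or per-tick auto detection, trace below feet to pick surface sounds and particles, with water override and velocity-scaled volume.
; For local players, timers scatter random traces that place capped, spaced surface-based ambient sounds, cull distant ones, and scale a wind loop by speed.
; Setup events supply all settings and maps.
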(event `self.ReceiveBeginPlay`
  ;[0.7813 0 1] Begin Play
  (`KismetSystemLibrary.Delay` 0.0)
  (`self.EventGetOwnerAsCharacter`)
  (`|ExecutionSequence`
    (:`then_0`
      ;[1 0 0.2344] Random stream
      (`KismetMathLibrary.SetRandomStreamSeed` (`self.RandomizeStream`) (`KismetMathLibrary.RandomIntegerInRange` 0 999)))))

(event `EventGetOwnerAsCharacter`
  (bind _debug_ (`self.Debug?`))
  ;[0 1 0.2734] Check if owner is character for future reference
  (bind _ascharacter (cast `Character` (`self.GetOwner`))
    (:`then`
      (set `self.OwnerCharacterReference` _ascharacter))
    (:`CastFailed`
      (`KismetSystemLibrary.PrintString` "Error - owner is not a character!" _debug_ _debug_))))

(event `EventSpawnSoundAttached`
  (params (Key :type "EPhysicalSurface Enum (by ref)") (Foot :type "Name (by ref)"))
  (bind _ownercharacterreference (`self.OwnerCharacterReference`))
  (bind (_value _returnvalue) (`BlueprintMapLibrary.Map_Find` (`self.SurfaceSounds`) Key))
  ;[1 0.5859 0] Spawn Sound
  (if _returnvalue
    (bind _returnvalue_2 (`GameplayStatics.SpawnSoundAttached` _value (select `bool` (`KismetSystemLibrary.IsValid` _ownercharacterreference) :`false` (`Actor.RootComponent` (`self.GetOwner`)) :`true` (`Character.Mesh` _ownercharacterreference) :!type "SceneComponent Object Reference") (`BlueprintMapLibrary.Map_Find` (`self.Feet`) Foot) (0.0 0.0 0.0) (struct) "SnapToTarget" false (* (`self.ReadVolumeValue` (`Actor.GetVelocity` (`self.GetOwner`))) (`self.FootstepVolumeMultiplier`)) 1.0 0.0 (`self.FootstepAttenuation`) (`self.FootstepConcurencySettings`)))
    (bind _output_get (set `self.FootstepSound` _returnvalue_2))
    ;;[0 0.9297 1] Parameters
    (`/Engine/EditorBlueprintResources/StandardMacros.IsValid` _output_get
      (:`Is Valid`
        (`AudioComponent.SetBoolParameter` _output_get "IsMale" (`self.Male?`))
        (`AudioComponent.SetBoolParameter` _output_get "Rattle" (`self.Rattle?`))))))

(event `SetupFootstepsDefaults`
  (params (VelocityToMinVolume :type "Float (double-precision)" :default 120.0) (VelocityMaxVolume :type "Float (double-precision)" :default 320.0) (`Male?` :type Boolean :default true) (`Rattle?` :type Boolean :default false) (VolumeMultiplier :type "Float (double-precision)" :default 1.0) (FootstepAttenuation :type "SoundAttenuation Object Reference") (FootstepConcurencySettings :type "SoundConcurrency Object Reference") (SurfaceSounds :type "Map of EPhysicalSurface Enum to SoundCue Object Reference") (SurfaceParticles :type "Map of EPhysicalSurface Enum to NiagaraSystem Object Reference") (`FootTraceComplex?` :type Boolean :default true) (FootstepsMinCycleInterval :type "Float (double-precision)" :default 0.25) (FootPartickleScale :type "Float (double-precision)" :default 0.5))
  ;[1 0 0.04687] Init setup
  (set `self.VelocityToMinVolume` VelocityToMinVolume)
  (set `self.VelocityMaxVolume` VelocityMaxVolume)
  (set `self.Male?` `Male?`)
  (set `self.Rattle?` `Rattle?`)
  (set `self.FootstepVolumeMultiplier` VolumeMultiplier)
  (set `self.FootstepAttenuation` FootstepAttenuation)
  (set `self.FootstepConcurencySettings` FootstepConcurencySettings)
  (set `self.SurfaceSounds` SurfaceSounds)
  (set `self.SurfaceParticles` SurfaceParticles)
  (set `self.FootTraceComplex?` `FootTraceComplex?`)
  (set `self.FootstepsMinCycleInterval` FootstepsMinCycleInterval)
  (set `self.FootPartickleScale` FootPartickleScale))

(event `SetupFeetDefinition`
  (params (Feet :type "Map of Name to Name"))
  ;[0 1 0.7891] Setup definition of feet bone shortcuts for notification
  (set `self.Feet` Feet))

(event `EventTryFootstep`
  (params (FootsavedName :type Name) (Mesh :type "SkeletalMeshComponent Object Reference"))
  (bind (_found_ _socketname) (`self.FindSocketFromName` FootsavedName))
  (bind _debug_ (`self.Debug?`))
  ;[0 1 0.8828] Init Footstep Event
  (if (and _found_ (`SceneComponent.DoesSocketExist` Mesh _socketname))
    ;[0.5234 0 1] Trace foot
    (bind (_returnvalue _outhit _surface) (`self.TraceFoot` _socketname Mesh 30.0))
    ;[0.1016 0 1] Debug error print
    (if _returnvalue
      (`self.EventInitFootstep` _outhit _surface _socketname)
      (else
        (`KismetSystemLibrary.PrintString` "DebugPrint! Nothing under the feet" _debug_ _debug_ (struct :`G` 0.66 :`B` 1.0 :`A` 1.0) 0.5)))))

(event `SetupAddOrUpdateSurface`
  (params (Surface :type "EPhysicalSurface Enum" :default "SurfaceType_Default") (sound :type "SoundCue Object Reference (by ref)") (niagaraParticle :type "NiagaraSystem Object Reference (by ref)"))
  ;[0 0.625 1] Alter the surface setup
  (`BlueprintMapLibrary.Map_Add` (`self.SurfaceSounds`) Surface sound)
  (`BlueprintMapLibrary.Map_Add` (`self.SurfaceParticles`) Surface niagaraParticle))

(event `EventSpawnParticle`
  (params (Key :type "EPhysicalSurface Enum (by ref)") (Transform :type "Transform Structure"))
  (bind (_value _returnvalue) (`BlueprintMapLibrary.Map_Find` (`self.SurfaceParticles`) Key))
  ;[1 0 0.2344] Spawn Particle
  (if _returnvalue
    (`NiagaraFunctionLibrary.SpawnSystemAtLocation` _value Transform_Location Transform_Rotation Transform_Scale true true "AutoRelease")))

(event `self.ReceiveTick`
  (params (DeltaSeconds :type "Float (single-precision)"))
  (bind _ownercharacterreference (`self.OwnerCharacterReference`))
  (bind _autofootstepsarray (`self.AutofootstepsArray`))
  (bind _debug_ (`self.Debug?`))
  ;[0 0.7187 1] Tick auto footsteps generator!
  ;;[0 1 0.7891] Auto footstep generator
  (if (`self.AutoFootRotation?`)
    (bind _values (`BlueprintMapLibrary.Map_Values` (`self.Feet`)))
    (for _array_element _values
      ;;[0 1 0.25] PerFoot tracing
      (if (`KismetMathLibrary.BooleanNOR` (`KismetArrayLibrary.Array_Contains` _autofootstepsarray _array_element) (== (`self.PreviousFoot`) _array_element))
        (`/Engine/EditorBlueprintResources/StandardMacros.IsValid` _ownercharacterreference
          (:`Is Valid`
            (bind (_returnvalue _outhit _surface) (`self.TraceFoot` _array_element (`Character.Mesh` _ownercharacterreference) (`self.AutofootstepTraceLen`)))
            (if _returnvalue
              (`KismetArrayLibrary.Array_AddUnique` _autofootstepsarray _array_element)
              (`self.EventInitFootstep` _outhit _surface _array_element)
              (set `self.PreviousFoot` _array_element)))
          (:`Is Not Valid`
            (`self.EventGetOwnerAsCharacter`)))))
    ;;[1 0 0.3047] Clear on stop
    (if (== (`KismetArrayLibrary.Array_Length` (`self.AutofootstepsArray`)) (`KismetArrayLibrary.Array_Length` _values))
      (if (not (`KismetMathLibrary.NearlyEqual_FloatFloat` (`KismetMathLibrary.VSize` (`Actor.GetVelocity` (`self.OwnerCharacterReference`))) 0.0 0.01))
        (`/Engine/EditorBlueprintResources/StandardMacros.Gate` false :!label _label
          (:`Exit`
            (`KismetArrayLibrary.Array_Clear` (`self.AutofootstepsArray`))
            (`KismetSystemLibrary.PrintString` "cleared auto foot array!" _debug_ _debug_ (struct :`G` 0.66 :`B` 1.0 :`A` 1.0) 0.5)
            (`|ExecutionSequence`
              (:`then_0`
                (goto _label :!via `Close`))
              (:`then_1`
                (`KismetSystemLibrary.Delay` (`self.FootstepsMinCycleInterval`))
                (goto _label :!via `Open`)))))))))

(event `EventInitFootstep`
  (params (Hit :type "HitResult Structure (by ref)") (Key :type "EPhysicalSurface Enum (by ref)") (Foot :type "Name (by ref)"))
  (bind (_bblockinghit _binitialoverlap _time _distance _location _impactpoint _normal) (`GameplayStatics.BreakHitResult` Hit))
  ;[1 0.2109 0] The actual footstep Event
  ;;[0 1 0.1328] Init footstep
  (`|ExecutionSequence`
    (:`then_0`
      ;;[1 0.5625 0] Spawn Sound for footsteps
      (if (`self.UseFootstepSounds?`)
        (`self.EventSpawnSoundAttached` (select `bool` (`self.InWater?`) :`false` Key :`true` (`self.WaterSurface`)) Foot)))
    (:`then_1`
      ;;[0 1 1] Spawn Partickle
      (if (`self.UseFootstepParticle?`)
        (`self.EventSpawnParticle` (select `bool` (`self.InWater?`) :`false` Key :`true` (`self.WaterSurface`)) (`KismetMathLibrary.MakeTransform` _impactpoint (`KismetMathLibrary.MakeRotFromZ` _normal) (* (`Actor.GetActorScale3D` (`self.GetOwner`)) (`self.FootPartickleScale`))))))
    (:`then_2`
      ;;[0 1 0.4844] Debug print
      (if (`self.Debug?`)
        (`KismetSystemLibrary.PrintText` (`|FormatText` "Footstep::     Surface:{0}   Foot:{1}" (`|GetEnumeratorNameAsString` Key) Foot) (`self.Debug?`) true (struct :`G` 0.66 :`B` 1.0 :`A` 1.0) 0.5)))))

(event `SetupAutoFootsteps`
  (params (`AutoFootRotation?` :type Boolean :default true) (AutofootstepTraceLen :type "Float (double-precision)" :default 15.0))
  ;[0.6641 1 0] Setup auto footsteps
  (set `self.AutoFootRotation?` `AutoFootRotation?`)
  (set `self.AutofootstepTraceLen` AutofootstepTraceLen))

(event `SetupWaterSurface`
  (params (WaterSurface :type "EPhysicalSurface Enum" :default "SurfaceType3"))
  ;[1 0.1641 0] In Water
  (set `self.WaterSurface` WaterSurface))

(event `SetupInWater`
  (params (`InWater?` :type Boolean))
  ;[1 0.1641 0] In Water
  (set `self.InWater?` `InWater?`))

(event `AddSountByName`
  (params (Key :type Name) (Value :type "SoundCue Object Reference"))
  ;[1 0 0.3984] speaking settings
  (`BlueprintMapLibrary.Map_Add` (`self.SoundByName`) Key Value))

(event `RemoveSountByName`
  (params (Key :type "Name (by ref)"))
  ;[1 0 0.3984] speaking settings
  (`BlueprintMapLibrary.Map_Remove` (`self.SoundByName`) Key))

(event `SetupSpeakingSettings`
  (params (SpeakingVolume :type "Float (double-precision)" :default 1.0) (SpeakingAttenuation :type "SoundAttenuation Object Reference") (TalkingConcurencySettings :type "SoundConcurrency Object Reference"))
  ;[0 1 0.7656] Setup
  (set `self.SpeakingVolume` SpeakingVolume)
  (set `self.SpeakingAttenuation` SpeakingAttenuation)
  (set `self.TalkingConcurencySettings` TalkingConcurencySettings))

(event `EventPlaySoundByKeyName`
  (params (Key :type "Name (by ref)"))
  (bind _returnvalue (`self.GetOwner`))
  (bind (_value _returnvalue_2) (`BlueprintMapLibrary.Map_Find` (`self.SoundByName`) Key))
  (bind (_returnvalue_location _returnvalue_rotation) (`KismetMathLibrary.BreakTransform` (`Actor.GetTransform` _returnvalue)))
  ;[1 0.1641 0] Play speaking sound by key name
  (if _returnvalue_2
    (bind _returnvalue_3 (`GameplayStatics.SpawnSoundAttached` _value (`Actor.RootComponent` _returnvalue) "None" _returnvalue_location _returnvalue_rotation "SnapToTarget" true (`self.SpeakingVolume`) 1.0 0.0 (`self.SpeakingAttenuation`) (`self.TalkingConcurencySettings`)))
    ;;[1 0 0.1875] Parameters
    (`AudioComponent.SetBoolParameter` _returnvalue_3 "IsMale" (`self.Male?`))
    (`AudioComponent.SetBoolParameter` _returnvalue_3 "Rattle" (`self.Rattle?`))))

(event `EventSpawnSoundDebug`
  (params (Location :type "Vector Structure") (Duration :type "Float (double-precision)"))
  ;[0.03125 0 1] Debug sounds
  (if (`self.Debug?`)
    (`KismetSystemLibrary.DrawDebugSphere` Location (`self.AmbientRange`) 24 (struct :`R` 1.0 :`G` 1.0 :`B` 1.0 :`A` 1.0) Duration 2.0)
    (`KismetSystemLibrary.DrawDebugSphere` Location 100.0 12 (struct :`R` 0.089927 :`G` 0.140379 :`B` 1.0 :`A` 1.0) Duration 3.0)))

(event `SpawnSingleAmbientSound`
  (params (Sound :type "SoundBase Object Reference") (Location :type "Vector Structure") (VolumeMultiplier :type "Float (double-precision)") (AttenuationSettings :type "SoundAttenuation Object Reference") (ConcurrencySettings :type "SoundConcurrency Object Reference"))
  ;[0 0.25 1] register
  ;;[1 0 0.07031] Only local player
  (if (`self.OwnerIsLocalPlayer`)
    (bind _returnvalue (`GameplayStatics.SpawnSoundAtLocation` Sound Location (struct) VolumeMultiplier 1.0 0.0 AttenuationSettings ConcurrencySettings false))
    ;;[0 1 1] spawn ambient sound
    (`KismetArrayLibrary.Array_Add` (`self.Ambients`) _returnvalue)
    (`self.EventSpawnSoundDebug` Location 1.0)))

(event `SetupAmbientTable`
  (params (AmbientSounds :type "Map of EPhysicalSurface Enum to SoundCue Object Reference"))
  ;[0 0.25 1] Change entire ambient table
  (set `self.AmbientSounds` AmbientSounds))

(event `EventClearCurrentSounds`
  (bind _ambients (`self.Ambients`))
  ;[0.7109 0 1] Clear existing sounds
  (for _array_element _ambients
    (`/Engine/EditorBlueprintResources/StandardMacros.IsValid` _array_element
      (:`Is Valid`
        (`self.K2_DestroyComponent` _array_element))))
  (`KismetArrayLibrary.Array_Clear` _ambients))

(event `SetupAmbientSettings`
  (params (`UseAmbientSound?` :type Boolean :default true) (AmbientVolume :type "Float (double-precision)" :default 1.0) (AmbientAttenuation :type "SoundAttenuation Object Reference") (AmbientConcurency :type "SoundConcurrency Object Reference") (AmbientRange :type "Float (double-precision)" :default 1000.0) (AmbientMax :type Integer :default 3) (MaxIdenticalAmbient :type Integer) (AmbientCheckIntervals :type "Float (double-precision)" :default 0.5) (AmbientTraceCount :type Integer :default 14) (MinDistanceBetweenAmbient :type "Float (double-precision)" :default 210.0))
  ;[1 0.6328 0] Setup
  (set `self.UseAmbientSound?` `UseAmbientSound?`)
  (set `self.AmbientVolume` AmbientVolume)
  (set `self.AmbientAttenuation` AmbientAttenuation)
  (set `self.AmbientConcurency` AmbientConcurency)
  (set `self.AmbientRange` AmbientRange)
  (set `self.AmbientMax` AmbientMax)
  (set `self.MaxIdenticalAmbient` MaxIdenticalAmbient)
  (set `self.AmbientCheckIntervals` AmbientCheckIntervals)
  (set `self.AmbientTraceCount` AmbientTraceCount)
  (set `self.MinDistanceBetweenAmbient` MinDistanceBetweenAmbient)
  (`KismetSystemLibrary.Delay` 0.2)
  ;;[0 1 0.3906] local player
  (if (and (`self.OwnerIsLocalPlayer`) (`self.UseAmbientSound?`))
    ;;[1 0 0.9375] Check ambient sounds
    (bind _returnvalue (`KismetSystemLibrary.K2_SetTimerDelegate` (delegate `EventFrameCheckAmbience`) (`self.AmbientCheckIntervals`) true))
    (set `self.AmbientCheckTimer` _returnvalue)))

(event `EventFrameCheckAmbience`
  (bind _ambients (`self.Ambients`))
  (bind _debug_ (`self.Debug?`))
  (bind _ownercharacterreference (`self.OwnerCharacterReference`))
  (bind _returnvalue (`KismetArrayLibrary.Array_Length` _ambients))
  (bind _returnvalue_2 (`Actor.K2_GetActorLocation` _ownercharacterreference))
  (bind _array (`|MakeArray` (`self.OwnerCharacterReference`) :!type "Actor Object Reference"))
  ;[0 1 0.6719] Check all sounds out of range
  ;;[0.5469 1 0] Try
  (if (> _returnvalue 0)
    (for (_array_element _array_index) _ambients
      ;;[1 0.5156 0] validity check
      (`/Engine/EditorBlueprintResources/StandardMacros.IsValid` _array_element
        (:`Is Valid`
          ;;[0 1 0.7656] Debug draw sounds
          (if (`self.Debug?`)
            (`self.EventSpawnSoundDebug` (`SceneComponent.K2_GetComponentLocation` _array_element) (`self.AmbientCheckIntervals`)))
          ;;[0.5469 0 1] Distance check
          (if (> (`KismetMathLibrary.Vector_Distance` (`SceneComponent.K2_GetComponentLocation` _array_element) (`Actor.K2_GetActorLocation` (`self.OwnerCharacterReference`))) (`self.AmbientRange`))
            ;;[1 0 0.5859] Destroy and remove. make way for new
            (`self.K2_DestroyComponent` _array_element)
            (`KismetArrayLibrary.Array_Remove` _ambients _array_index)))
        (:`Is Not Valid`
          (`KismetArrayLibrary.Array_Remove` _ambients _array_index)))))
  ;[0.5703 1 0] Finish
  (`KismetSystemLibrary.PrintText` (`|FormatText` "Ambient sounds: {0}" _returnvalue) _debug_ _debug_)
  (if (< (`KismetArrayLibrary.Array_Length` (`self.Ambients`)) (`self.AmbientMax`))
    ;[1 0.2109 0] Make ignore list
    (`KismetArrayLibrary.Array_Append` _array (`Actor.GetAttachedActors` (`self.OwnerCharacterReference`) true))
    ;[0.1719 1 0] Find surface
    (for _ (range (+ (`self.AmbientTraceCount`) 1))
      (bind (_outhit _returnvalue_3) (`KismetSystemLibrary.LineTraceSingle` _returnvalue_2 (+ _returnvalue_2 (* (`KismetMathLibrary.Conv_RotatorToVector` (`KismetMathLibrary.ComposeRotators` (`Actor.K2_GetActorRotation` _ownercharacterreference) (`KismetMathLibrary.RandomRotatorFromStream` false (`self.RandomizeStream`)))) (`self.AmbientRange`))) "TraceTypeQuery1" false _array (select `bool` (`self.Debug?`) :`true` "ForDuration" :!type "EDrawDebugTrace Enum") true (struct :`R` 1.0 :`A` 1.0) (struct :`G` 1.0 :`A` 1.0) 1.0))
      ;[0 1 0.7656] Can spawn sound?
      (if _returnvalue_3
        (bind (_bblockinghit _binitialoverlap _time _distance _location _impactpoint _normal _impactnormal _physmat) (`GameplayStatics.BreakHitResult` _outhit))
        (bind (_value _returnvalue_4) (`BlueprintMapLibrary.Map_Find` (`self.AmbientSounds`) (`PhysicalMaterial.SurfaceType` _physmat)))
        (if _returnvalue_4
          (bind _spawnsound_ (`self.AlreadyPlayingSound?` _value (`self.MaxIdenticalAmbient`) _impactpoint (`self.MinDistanceBetweenAmbient`)))
          (if _spawnsound_
            ;[0.7578 1 0] Spawn single sound
            (`self.SpawnSingleAmbientSound` _value _impactpoint (`self.AmbientVolume`) (`self.AmbientAttenuation`) (`self.AmbientConcurency`))
            (break)))))))

(event `SetupWind`
  (params (`UseDynamicWind?` :type Boolean :default false) (Windsound :type "SoundCue Object Reference") (WindWeatherVolumeMulti :type "Float (double-precision)" :default 1.0) (MaxWindAtVelocity :type "Float (double-precision)" :default 1200.0) (RefreshRate :type "Float (double-precision)" :default 0.2))
  ;[0.6406 1 0] Setup
  (bind _output_get (set `self.UseDynamicWind?` `UseDynamicWind?`))
  (set `self.Windsound` Windsound)
  (set `self.WindWeatherVolumeMulti` WindWeatherVolumeMulti)
  (set `self.MaxWindAtVelocity` MaxWindAtVelocity)
  (set `self.WindRefreshRate` RefreshRate)
  (`self.InitOrStopWind` (not _output_get)))

(event `EventUpdateWind`
  (bind _windsoundcomponent (`self.WindSoundComponent`))
  (bind _debug_ (`self.Debug?`))
  ;[1 0.8672 0] Update
  ;;[0 1 0.2969] Timer update event
  (`/Engine/EditorBlueprintResources/StandardMacros.IsValid` _windsoundcomponent
    (:`Is Valid`
      (`AudioComponent.SetVolumeMultiplier` _windsoundcomponent (* (`self.AmbientVolume`) (`KismetMathLibrary.MapRangeClamped` (`KismetMathLibrary.Abs` (`KismetMathLibrary.VSize` (`Actor.GetVelocity` (`self.OwnerCharacterReference`)))) 0.0 (`self.MaxWindAtVelocity`) 0.5 1.0) (`self.WindWeatherVolumeMulti`))))
    (:`Is Not Valid`
      ;;[0.8516 1 0] stop timer
      (`KismetSystemLibrary.K2_ClearAndInvalidateTimerHandle` (stale `InitOrStopWind` _output_get))
      (`KismetSystemLibrary.PrintString` "Something went wrong and wind stopped working!" _debug_ _debug_))))

(event `InitOrStopWind`
  (params (`Pause?` :type Boolean))
  (bind _ownercharacterreference (`self.OwnerCharacterReference`))
  (bind (_returnvalue_location _returnvalue_rotation) (`KismetMathLibrary.BreakTransform` (`Actor.GetTransform` _ownercharacterreference)))
  ;[0.8984 0 1] Init
  (if `Pause?`
    (`KismetSystemLibrary.K2_ClearAndInvalidateTimerHandle` (`self.Windtimer`))
    (else
      (`KismetSystemLibrary.Delay` 0.2)
      ;[0 0.7422 1] Use wind system? Only local player owner
      (if (and (`self.UseDynamicWind?`) (`self.OwnerIsLocalPlayer`))
        ;[0.6406 0 1] pawn wind component
        (bind _returnvalue (`GameplayStatics.SpawnSoundAttached` (`self.Windsound`) (`Actor.RootComponent` _ownercharacterreference) "None" _returnvalue_location _returnvalue_rotation "SnapToTarget" true (`self.AmbientVolume`) 1.0 0.0 "/Game/AGR/Audio/AmbientSoundAttenuation.AmbientSoundAttenuation" "/Game/AGR/Audio/Ambientconcurency.AmbientConcurency"))
        (set `self.WindSoundComponent` _returnvalue)
        ;[1 0.8672 0] Update
        ;;[0 1 0.5781] Start timer
        (bind _returnvalue_2 (`KismetSystemLibrary.K2_SetTimerDelegate` (delegate `EventUpdateWind`) (`self.WindRefreshRate`) true))
        (bind _output_get (set `self.Windtimer` _returnvalue_2))))))

(fn `AlreadyPlayingSound?`
  (params (ObjectCheck :type "Object Object Reference") (MaxSameSounds :type Integer :default 1) (`Proximity location` :type "Vector Structure") (MinDistance :type "Float (double-precision)"))
  (returns (`SpawnSound?` :type Boolean) (TimesPlaying :type Integer))
  (locals (AlreadyPlaying :type Integer) (ShouldNotSpawn :type Boolean))
  (for _array_element (`self.Ambients`)
    (`/Engine/EditorBlueprintResources/StandardMacros.IsValid` _array_element
      (:`Is Valid`
        (if (== ObjectCheck (`AudioComponent.Sound` _array_element))
          (bind _result (`/Engine/EditorBlueprintResources/StandardMacros.IncrementInt` (`local.AlreadyPlaying`))
            (:`  `
              (bind _returnvalue (< (`KismetMathLibrary.Vector_Distance` (`SceneComponent.K2_GetComponentLocation` _array_element) `Proximity location`) MinDistance))
              (if (or _returnvalue (>= _result MaxSameSounds))
                (set `local.ShouldNotSpawn` true :!label _label)
                (break))))
          (elif _returnvalue
            (goto _label))))))
  (return (not (`local.ShouldNotSpawn`)) (`local.AlreadyPlaying`)))

(fn `FindSocketFromName`
  (params (StoredFootName :type Name))
  (returns (`Found?` :type Boolean) (SocketName :type Name))
  (bind (_value _returnvalue) (`BlueprintMapLibrary.Map_Find` (`self.Feet`) StoredFootName))
  (return _returnvalue _value))

(fn `OwnerIsLocalPlayer`
  (returns (ReturnValue :type Boolean))
  (bind _ownercharacterreference (`self.OwnerCharacterReference`))
  (`/Engine/EditorBlueprintResources/StandardMacros.IsValid` _ownercharacterreference
    (:`Is Valid`
      (return (and (`Pawn.IsLocallyControlled` _ownercharacterreference) (`Pawn.IsPlayerControlled` _ownercharacterreference))))
    (:`Is Not Valid`
      (return false))))

(fn `ReadVolumeValue`
  (params (InVelocity :type "Vector Structure"))
  (returns (OutVolume :type "Float (double-precision)"))
  (return (`KismetMathLibrary.MapRangeClamped` (`KismetMathLibrary.VSize` InVelocity) (`self.VelocityToMinVolume`) (`self.VelocityMaxVolume`) 0.1 1.0)))

(fn `TraceFoot`
  (params (TraceSocketName :type Name) (Mesh :type "SkeletalMeshComponent Object Reference") (TraceLen :type "Float (double-precision)"))
  (returns (ReturnValue :type Boolean) (OutHit :type "HitResult Structure") (Surface :type "EPhysicalSurface Enum") (ImpactPoint :type "Vector Structure"))
  (bind _returnvalue (`SceneComponent.GetSocketLocation` Mesh TraceSocketName))
  ;[1 0.7969 0] Trace
  (bind (_outhit _returnvalue_2) (`KismetSystemLibrary.LineTraceSingle` _returnvalue (+ _returnvalue (`KismetMathLibrary.MakeVector` 0.0 0.0 (* -1 TraceLen))) "TraceTypeQuery1" (`self.FootTraceComplex?`) (`|MakeArray` (`self.GetOwner`)) (select `bool` (`self.Debug?`) :`true` "ForDuration" :!type "EDrawDebugTrace Enum") true (struct :`R` 1.0 :`A` 1.0) (struct :`G` 1.0 :`A` 1.0) 1.0))
  ;[1 0 0] Got any hit
  (if _returnvalue_2
    ;[0.4062 1 0] Debug Draw
    (if (`self.Debug?`)
      (bind (_bblockinghit _binitialoverlap _time _distance _location _impactpoint _normal _impactnormal _physmat) (`GameplayStatics.BreakHitResult` _outhit))
      (`KismetSystemLibrary.DrawDebugSphere` _impactpoint 25.0 12 (struct :`G` 0.598958 :`B` 0.223925 :`A` 1.0) 0.5 1.0))
    (return _returnvalue_2 _outhit (`PhysicalMaterial.SurfaceType` _physmat) _impactpoint)
    (else
      (return false (struct) "SurfaceType_Default" (0.0 0.0 0.0)))))