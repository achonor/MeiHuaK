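; AGR AI component that starts movement behavior trees for its owning actor and randomizes a wait cooldown.
; The setup event runs a supplied behavior tree asset on the owner's AI controller and prints whether it started.
; A separate event picks a random cooldown between custom minimum and maximum values, stores it as the current cooldown and prints it.
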(event `SetupRunMovementBT`
  (params (BTAsset :type "BehaviorTree Object Reference"))
  (bind _returnvalue (`AIController.RunBehaviorTree` (`AIBlueprintHelperLibrary.GetAIController` (`self.GetOwner`)) BTAsset))
  (if _returnvalue
    (`KismetSystemLibrary.PrintString` "Started Behavior tree for walking!")
    (else
      (`KismetSystemLibrary.PrintString` "Failed to start Behavior tree for walking!"))))

(event `EventRandomizeWait`
  (bind _output_get (set `self.CurrentCooldown` (`KismetMathLibrary.RandomFloatInRange` (`self.CustomCooldownMin`) (`self.CustomCooldownMax`))))
  (`KismetSystemLibrary.PrintString` (`KismetStringLibrary.Conv_DoubleToString` _output_get)))