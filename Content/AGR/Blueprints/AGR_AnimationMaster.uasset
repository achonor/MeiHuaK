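; Character component that manages networked animation state: poses, aim offset, turn modes, first-person flag, montages and ragdoll.
; Setup events relay most settings through server events, and RepNotifies apply rotation and ragdoll changes.
; Tick derives aim from a camera trace or control rotation, relays it, and uses it for turn-at-angle with tolerance.
; Ragdoll toggles pelvis-down physics and snapshots the pose on exit; its capsule-follow logic is disconnected.
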(event `self.ReceiveBeginPlay`
  ;[0.07812 1 0] Start - references
  (`self.EventRedoCasts`)
  (`KismetSystemLibrary.Delay` 0.0)
  (`self.EventRedoCasts`))

(event `ServerAimOffset`
  (params (Aim :type "Rotator Structure"))
  ;[0 1 0.282] TICK
  (`self.MultiAimOffset` Aim))

(event `MultiAimOffset`
  (params (AimOffset :type "Rotator Structure"))
  (bind _characterreference (`self.CharacterReference`))
  ;[0 1 0.282] TICK
  (`/Engine/EditorBlueprintResources/StandardMacros.IsValid` _characterreference
    (:`Is Valid`
      (if (not (and (`Pawn.IsLocallyControlled` _characterreference) (`Pawn.IsPlayerControlled` _characterreference)))
        (set `self.AimOffset` AimOffset)))))

(event `self.ReceiveTick`
  (params (DeltaSeconds :type "Float (single-precision)"))
  (bind _returnvalue (`GameplayStatics.GetPlayerCameraManager` 0))
  (bind _characterreference (`self.CharacterReference`))
  (bind _debug_ (`self.Debug?`))
  (bind _charmovementcomponent (`self.CharMovementComponent`))
  (bind _returnvalue_2 (`PlayerCameraManager.GetCameraLocation` _returnvalue))
  (bind _returnvalue_3 (`KismetMathLibrary.FClamp` (`self.TurnTolerance`) 1.0 90.0))
  (bind _mesh (`Character.Mesh` (`self.CharacterReference`)))
  (bind _returnvalue_4 (`SceneComponent.GetSocketLocation` _mesh "head"))
  (bind _returnvalue_5 (`SceneComponent.GetSocketLocation` _mesh "ik_hand_gun"))
  (bind (_returnvalue_roll _returnvalue_pitch _returnvalue_yaw) (`KismetMathLibrary.BreakRotator` (`KismetMathLibrary.NormalizedDeltaRotator` (`self.AimOffset`) (`Actor.K2_GetActorRotation` (`self.CharacterReference`)))))
  (bind _returnvalue_6 (`SceneComponent.GetSocketLocation` (`Character.Mesh` (`self.CharacterReference`)) (select `bool` (== (`self.AimOffsetTag`) (struct :`TagName` "Animation.AimOffset.AimAt")) :`false` "spine_03" :`true` "ik_hand_gun" :!type "Name")))
  (bind _returnvalue_7 (+ _returnvalue_2 (* (`Actor.GetActorForwardVector` _returnvalue) 10000.0)))
  ;[0 1 0.282] TICK
  (`|ExecutionSequence`
    (:`then_0`
      (if (`Pawn.IsLocallyControlled` _characterreference)
        (if (and (`Pawn.IsPlayerControlled` _characterreference) (`self.CameraBasedAim?`))
          (bind (_outhit _returnvalue_8) (`KismetSystemLibrary.LineTraceSingle` _returnvalue_2 _returnvalue_7 "TraceTypeQuery1" true (`|MakeArray` (`self.GetOwner`)) (select `bool` (`self.Debug?`) :`true` "ForOneFrame" :!type "EDrawDebugTrace Enum")))
          (if _returnvalue_8
            (set `self.LookAtLocation` (`.Location` (`GameplayStatics.BreakHitResult` _outhit)))
            (bind _output_get (set `self.AimOffset` (`KismetMathLibrary.FindLookAtRotation` _returnvalue_6 (`.Location` (`GameplayStatics.BreakHitResult` _outhit)))))
            (`self.ServerAimOffset` _output_get)
            (if _debug_
              (`KismetSystemLibrary.DrawDebugLine` _returnvalue_4 (`.Location` (`GameplayStatics.BreakHitResult` _outhit)) (struct :`G` 0.5 :`B` 0.5 :`A` 1.0) 0.0 1.0)
              (`KismetSystemLibrary.DrawDebugLine` _returnvalue_5 (`.Location` (`GameplayStatics.BreakHitResult` _outhit)) (struct :`R` 0.5 :`B` 0.5 :`A` 1.0) 0.0 1.0))
            (else
              (bind _output_get_2 (set `self.AimOffset` (`KismetMathLibrary.FindLookAtRotation` _returnvalue_6 _returnvalue_7)))
              (`self.ServerAimOffset` _output_get_2)
              (if _debug_
                (`KismetSystemLibrary.DrawDebugLine` _returnvalue_4 _returnvalue_7 (struct :`G` 0.5 :`B` 0.5 :`A` 1.0) 0.0 1.0)
                (`KismetSystemLibrary.DrawDebugLine` _returnvalue_5 _returnvalue_7 (struct :`R` 0.5 :`B` 0.5 :`A` 1.0) 0.0 1.0))))
          (else
            (bind _output_get_3 (set `self.AimOffset` (`Pawn.GetControlRotation` _characterreference)))
            (`self.ServerAimOffset` _output_get_3)))))
    (:`then_1`
      (if (== (`self.RotateTurnTag`) (struct :`TagName` "Animation.Turn.DesiredRotAtAngle"))
        (if (or (> (`KismetMathLibrary.Abs` _returnvalue_yaw) (`self.TurnStartAngle`)) (> (`KismetMathLibrary.VSize` (`Actor.GetVelocity` (`self.CharacterReference`))) 50.0))
          (set `CharacterMovementComponent.bUseControllerDesiredRotation` true _charmovementcomponent)
          (elif (`KismetMathLibrary.InRange_FloatFloat` _returnvalue_yaw (/ _returnvalue_3 -1.0) (/ _returnvalue_3 1.0))
            (set `CharacterMovementComponent.bUseControllerDesiredRotation` false _charmovementcomponent)))))
    (:`then_2`
      (if (`self.IsRagdolling`)
        _))))

(event `EventRedoCasts`
  ;[0.3594 0 1] Cast and store references
  (bind _ascharacter (cast `Character` (`self.GetOwner`)))
  (bind _output_get (set `self.CharacterReference` _ascharacter))
  (set `self.CharMovementComponent` (`Character.CharacterMovement` _output_get)))

(event `ServerPlayMontage`
  (params (MontageToPlay :type "AnimMontage Object Reference") (PlayRate :type "Float (double-precision)") (StartingSection :type Name))
  ;[0 1 0.7422] Multiplayer Animation Montage
  (`Character.PlayAnimMontage` (`self.CharacterReference`) MontageToPlay PlayRate StartingSection)
  (`self.MultiPlayMontage` MontageToPlay PlayRate StartingSection))

(event `PlayNetworkedMontage`
  (params (Montage :type "AnimMontage Object Reference") (PlayRate :type "Float (double-precision)" :default 1.0) (StartingSection :type Name))
  ;[0 1 0.7422] Multiplayer Animation Montage
  (if (`self.LocalControlled`)
    (`Character.PlayAnimMontage` (`self.CharacterReference`) Montage PlayRate StartingSection)
    (`self.ServerPlayMontage` Montage PlayRate StartingSection)))

(event `MultiPlayMontage`
  (params (AnimMontage :type "AnimMontage Object Reference") (InPlayRate :type "Float (double-precision)") (StartSectionName :type Name))
  ;[0 1 0.7422] Multiplayer Animation Montage
  (if (not (`self.LocalControlled`))
    (`Character.PlayAnimMontage` (`self.CharacterReference`) AnimMontage InPlayRate StartSectionName)))

(event `EventSetupFirstPerson`
  (params (`IsFirstPersonView?` :type Boolean))
  ;[0.1953 1 0] FP View
  (bind _output_get (set `self.IsFirstPersonView?` `IsFirstPersonView?`))
  (`self.OnFPPChange` _output_get))

(event `EventSetupBasePose`
  (params (BasePoseTag :type "GameplayTag Structure"))
  ;[1 0.375 0] Set Base pose
  (set `self.BasePoseTag` BasePoseTag)
  (`self.ServerSetBasePose` BasePoseTag))

(event `ServerSetBasePose`
  (params (BasePoseTag :type "GameplayTag Structure"))
  ;[1 0.375 0] Set Base pose
  (set `self.BasePoseTag` BasePoseTag))

(event `EventSetupOverlayPose`
  (params (OverlayTag :type "GameplayTag Structure"))
  ;[1 0 0.8203] Set OverlayPose
  (set `self.OverlayTag` OverlayTag)
  (`self.ServerSetOverlayPose` OverlayTag))

(event `ServerSetOverlayPose`
  (params (OverlayTag :type "GameplayTag Structure"))
  ;[1 0 0.8203] Set OverlayPose
  (set `self.OverlayTag` OverlayTag))

(event `ServerSetRotation`
  (params (RotateTurnTag :type "GameplayTag Structure" :default (struct)) (RotationSpeed :type "Float (double-precision)" :default 380.0) (TurnStartAngle :type "Float (double-precision)" :default 90.0) (TurnTolerance :type "Float (double-precision)" :default 5.0))
  ;[0 0.0625 1] Change Rotation
  (set `self.RotateTurnTag` RotateTurnTag)
  (set `self.RotationSpeed` RotationSpeed)
  (set `self.TurnStartAngle` TurnStartAngle)
  (set `self.TurnTolerance` TurnTolerance))

(event `EventSetupTurnRotation`
  (params (RotationType :type "GameplayTag Structure") (RotationSpeed :type "Float (double-precision)") (TurnStartAngle :type "Float (double-precision)") (TurnTolerance :type "Float (double-precision)"))
  ;[0 0.0625 1] Change Rotation
  (set `self.RotateTurnTag` RotationType)
  (set `self.RotationSpeed` RotationSpeed)
  (set `self.TurnStartAngle` TurnStartAngle)
  (set `self.TurnTolerance` TurnTolerance)
  (`self.ServerSetRotation` RotationType RotationSpeed TurnStartAngle TurnTolerance))

(event `ServerSetAimOffset`
  (params (AimOffsetTag :type "GameplayTag Structure") (AimOffsetSpeed :type "Float (double-precision)" :default 6.0) (AimOffsetClampAbsValue :type "Float (double-precision)") (`CameraBased?` :type Boolean) (AimClamp :type "GameplayTag Structure" :default (struct :`TagName` "Animation.AimClamp.Nearest")))
  ;[0 1 0.5547] Set aim offset
  (set `self.AimOffsetTag` AimOffsetTag)
  (set `self.AimOffsetSpeed` AimOffsetSpeed)
  (set `self.AimOffsetClampAbsValue` AimOffsetClampAbsValue)
  (set `self.CameraBasedAim?` `CameraBased?`)
  (set `self.AimClamp` AimClamp))

(event `EventSetupAimOffset`
  (params (AimOffsetTag :type "GameplayTag Structure" :default (struct)) (AimOffsetSpeed :type "Float (double-precision)" :default 6.0) (AimOffsetClampAbsValue :type "Float (double-precision)" :default 90.0) (`CameraBasedAim?` :type Boolean) (AimClamp :type "GameplayTag Structure"))
  ;[0 1 0.5547] Set aim offset
  (set `self.AimOffsetTag` AimOffsetTag)
  (set `self.AimOffsetSpeed` AimOffsetSpeed)
  (set `self.AimOffsetClampAbsValue` AimOffsetClampAbsValue)
  (set `self.CameraBasedAim?` `CameraBasedAim?`)
  (set `self.AimClamp` AimClamp)
  (`self.ServerSetAimOffset` AimOffsetTag AimOffsetSpeed AimOffsetClampAbsValue `CameraBasedAim?` AimClamp))

(event `ServerRagdoll`
  (params (Condition :type Boolean))
  ;[0.7812 1 0] Ragdoll
  (`self.MultiRagdoll` Condition))

(event `MultiRagdoll`
  (params (`Start?` :type Boolean))
  (bind _characterreference (`self.CharacterReference`))
  (bind _mesh (`Character.Mesh` (`self.CharacterReference`)))
  (bind _mesh_2 (`Character.Mesh` _characterreference))
  (bind _capsulecomponent (`Character.CapsuleComponent` _characterreference))
  ;[0.7812 1 0] Ragdoll
  (bind _output_get (set `self.IsRagdolling` `Start?`))
  (if (not _output_get)
    ;;[0.7812 0 1] End
    (`AnimInstance.SavePoseSnapshot` (`SkeletalMeshComponent.GetAnimInstance` _mesh) "RagdollPose" :!label _label)
    (`SkeletalMeshComponent.SetAllBodiesSimulatePhysics` _mesh_2 false)
    (`PrimitiveComponent.SetCollisionEnabled` _capsulecomponent "QueryAndPhysics")
    (`CharacterMovementComponent.SetMovementMode` (`self.CharMovementComponent`) "MOVE_Walking" 0)
    (`PrimitiveComponent.SetCollisionObjectType` _mesh "ECC_Pawn")
    (`SceneComponent.K2_AttachToComponent` _mesh_2 _capsulecomponent "None" "SnapToTarget" "SnapToTarget" "KeepWorld" false)
    (`SceneComponent.K2_SetRelativeLocationAndRotation` _mesh_2 (`KismetMathLibrary.MakeVector` 0.0 0.0 (* (`CapsuleComponent.CapsuleHalfHeight` _capsulecomponent) -1.0)) (struct :`Yaw` -90.0) false false)
    (`self.OnRagdollEnd`)))

(event `Ragdoll`
  (params (`Start?` :type Boolean) (PhysicsBlendWeight :type "Float (double-precision)" :default 1.0))
  (bind _characterreference (`self.CharacterReference`))
  (bind _pelvisbonename (`self.PelvisBoneName`))
  (bind _mesh (`Character.Mesh` _characterreference))
  ;[0.7812 1 0] Ragdoll
  (bind _output_get (set `self.IsRagdolling` `Start?`))
  (if _output_get
    ;;[0 0.2969 1] Simulate
    (`self.ServerRagdoll` `Start?`)
    (`SkeletalMeshComponent.SetAllBodiesBelowSimulatePhysics` _mesh _pelvisbonename true true)
    (`SkeletalMeshComponent.SetAllBodiesBelowPhysicsBlendWeight` _mesh _pelvisbonename PhysicsBlendWeight false true)
    (`SceneComponent.K2_DetachFromComponent` _mesh "KeepWorld" "KeepWorld" "KeepWorld" false)
    (`KismetSystemLibrary.Delay` 0.2)
    (`CharacterMovementComponent.SetMovementMode` (`self.CharMovementComponent`) "MOVE_Custom" 0)
    (`PrimitiveComponent.SetCollisionEnabled` (`Character.CapsuleComponent` _characterreference) "NoCollision")
    (`PrimitiveComponent.SetCollisionObjectType` _mesh "ECC_PhysicsBody")
    (`self.OnRagdollStart`)
    (else
      ;;[0.7812 0 1] End
      (`self.ServerRagdoll` `Start?`)
      (goto _label))))

(event `SetupPelvisBoneName`
  (params (PelvisBoneName :type Name :default "pelvis"))
  ;[1 0.3281 0] Setup ragdoll varaibles
  (`self.ServerPelvisBone` PelvisBoneName))

(event `ServerPelvisBone`
  (params (PelvisBoneName :type Name))
  ;[1 0.3281 0] Setup ragdoll varaibles
  (set `self.PelvisBoneName` PelvisBoneName))

(event `SetupIkValues`
  (params (AdditiveAlpha :type "Float (double-precision)" :default 1.0) (IkScale :type "Float (double-precision)" :default 1.0))
  ;[0 1 0.5547] Setup Ik Values
  (set `self.AdditiveAlpha` AdditiveAlpha)
  (set `self.IkScale` IkScale))

(fn `FacingDirection`
  (returns (`Up?` :type Boolean))
  (bind (_returnvalue_x _returnvalue_y _returnvalue_z) (`KismetMathLibrary.BreakVector` (`KismetMathLibrary.GetForwardVector` (`SceneComponent.GetSocketRotation` (`Character.Mesh` (`self.CharacterReference`)) (`self.PelvisBoneName`)))))
  (return (> _returnvalue_z 0.0)))

(fn `IsFirstPerson?`
  (returns (`FppView?` :type Boolean))
  (return (`self.IsFirstPersonView?`)))

(fn `LocalControlled`
  (returns (IsLocalPlayer :type Boolean))
  (return (`Pawn.IsLocallyControlled` (`self.CharacterReference`))))

(fn `OnRep_IsRagdolling`
  (bind _isragdolling (`self.IsRagdolling`))
  (`self.Ragdoll` _isragdolling (select `bool` _isragdolling :`true` 1.0 :!type "Float (single-precision)")))

(fn `OnRep_RotateTurnTag`
  (bind _charmovementcomponent (`self.CharMovementComponent`))
  (bind _charmovementcomponent_2 (`self.CharMovementComponent`))
  (bind _charmovementcomponent_3 (`self.CharMovementComponent`))
  (bind _charmovementcomponent_4 (`self.CharMovementComponent`))
  (bind _charmovementcomponent_5 (`self.CharMovementComponent`))
  (`/Engine/EditorBlueprintResources/StandardMacros.IsValid` (`self.CharacterReference`)
    (:`Is Valid`
      (`/Engine/EditorBlueprintResources/StandardMacros.IsValid` (`self.CharMovementComponent`)
        (:`Is Valid`
          (`|SwitchGameplayTag` (`self.RotateTurnTag`)
            (:`Animation.Turn.NONE`
              (set `Pawn.bUseControllerRotationYaw` false (`self.CharacterReference`))
              (set `CharacterMovementComponent.bOrientRotationToMovement` false _charmovementcomponent_4)
              (set `CharacterMovementComponent.bUseControllerDesiredRotation` false _charmovementcomponent_4))
            (:`Animation.Turn.CharacterRotYaw`
              (set `Pawn.bUseControllerRotationYaw` true (`self.CharacterReference`))
              (set `CharacterMovementComponent.bOrientRotationToMovement` false _charmovementcomponent_2)
              (set `CharacterMovementComponent.bUseControllerDesiredRotation` false _charmovementcomponent_2))
            (:`Animation.Turn.DesiredRotation`
              (set `Pawn.bUseControllerRotationYaw` false (`self.CharacterReference`))
              (set `CharacterMovementComponent.bOrientRotationToMovement` false _charmovementcomponent_3)
              (set `CharacterMovementComponent.bUseControllerDesiredRotation` true _charmovementcomponent_3))
            (:`Animation.Turn.RotToMovement`
              (set `Pawn.bUseControllerRotationYaw` false (`self.CharacterReference`))
              (set `CharacterMovementComponent.bOrientRotationToMovement` true _charmovementcomponent)
              (set `CharacterMovementComponent.bUseControllerDesiredRotation` false _charmovementcomponent))
            (:`Animation.Turn.DesiredRotAtAngle`
              (set `Pawn.bUseControllerRotationYaw` false (`self.CharacterReference`))
              (set `CharacterMovementComponent.bOrientRotationToMovement` false _charmovementcomponent_5)
              (set `CharacterMovementComponent.bUseControllerDesiredRotation` false _charmovementcomponent_5))))))))

(fn `OnRep_RotationSpeed`
  (bind _characterreference (`self.CharacterReference`))
  (`/Engine/EditorBlueprintResources/StandardMacros.IsValid` _characterreference
    (:`Is Valid`
      (set `CharacterMovementComponent.RotationRate` (`KismetMathLibrary.MakeRotator` 0.0 0.0 (`self.RotationSpeed`)) (`Character.CharacterMovement` _characterreference)))))