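; AGR_LIBRARY is a Blueprint library of gameplay helpers for tracing, target selection and value regeneration.
; Forward trace casts a line along a component's forward vector by channel or object type, using StartStop for endpoints.
; Sphere trace gathers overlapping actors around an origin, while two pickers choose a target from an array by highest dot product or shortest distance.
; The regen helper changes a by-ref float per second with delta time and clamping.
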(fn `AGR_BestClosestTarget`
  (params (Origin :type "Actor Object Reference") (Targets :type "Array of Actor Object Reference"))
  (returns (Target :type "Actor Object Reference") (Distance :type "Float (double-precision)"))
  (locals (BestLocalDistns :type "Float (double-precision)" :default 100000.0) (BestLocalTrgt :type "Actor Object Reference"))
  (for _array_element Targets
    (bind _returnvalue (`KismetMathLibrary.Vector_Distance` (`Actor.K2_GetActorLocation` Origin) (`Actor.K2_GetActorLocation` _array_element)))
    (if (< _returnvalue (`local.BestLocalDistns`))
      (set `local.BestLocalDistns` _returnvalue)
      (set `local.BestLocalTrgt` _array_element)))
  (return (`local.BestLocalTrgt`) (`local.BestLocalDistns`)))

(fn `AGR_BestDotTarget`
  (params (ActorStart :type "Actor Object Reference") (Targets :type "Array of Actor Object Reference"))
  (returns (BestTarget :type "Actor Object Reference") (BestDot :type "Float (double-precision)"))
  (locals (BestDotProduct :type "Float (double-precision)" :default -1.0) (Target :type "Actor Object Reference"))
  (for _array_element Targets
    (bind _returnvalue (`Actor.GetDotProductTo` ActorStart _array_element))
    (if (>= _returnvalue (`local.BestDotProduct`))
      (set `local.BestDotProduct` _returnvalue)
      (set `local.Target` _array_element)))
  (return (`local.Target`) (`local.BestDotProduct`)))

(fn `AGR_ForwardTrace`
  (params (Component :type "SceneComponent Object Reference") (`ByChannel?` :type Boolean :default true) (TraceChannel :type "ETraceTypeQuery Enum" :default "TraceTypeQuery1") (ObjectTypes :type "Array of EObjectTypeQuery Enum (by ref)") (`TraceComplex?` :type Boolean) (TraceDistance :type "Float (double-precision)" :default 5000.0) (ActorsToIgnore :type "Array of Actor Object Reference (by ref)") (DrawDebugType :type "EDrawDebugTrace Enum" :default "None") (`IgnoreSelf?` :type Boolean :default true) (TraceColor :type "LinearColor Structure" :default (struct :`R` 1.0 :`A` 1.0)) (TraceHitColor :type "LinearColor Structure" :default (struct :`G` 1.0 :`A` 1.0)) (DrawTime :type "Float (double-precision)" :default 1.0))
  (returns (`GotHit?` :type Boolean) (OutHit :type "HitResult Structure"))
  (bind _returnvalue (`SceneComponent.K2_GetComponentLocation` Component))
  (bind _returnvalue_2 (+ _returnvalue (* (`SceneComponent.GetForwardVector` Component) TraceDistance)))
  (if `ByChannel?`
    (bind (_outhit _returnvalue_3) (`KismetSystemLibrary.LineTraceSingle` Component _returnvalue _returnvalue_2 TraceChannel `TraceComplex?` ActorsToIgnore DrawDebugType `IgnoreSelf?` TraceColor TraceHitColor DrawTime))
    (if _returnvalue_3
      (return true _outhit)
      (else
        (return false (`GameplayStatics.MakeHitResult` false false 0.0 0.0 (0.0 0.0 0.0) (0.0 0.0 0.0) (0.0 0.0 1.0) (0.0 0.0 1.0) null null null "None" 0 0 _returnvalue _returnvalue_2))))
    (else
      (bind (_outhit_2 _returnvalue_4) (`KismetSystemLibrary.LineTraceSingleForObjects` Component _returnvalue _returnvalue_2 ObjectTypes `TraceComplex?` ActorsToIgnore DrawDebugType `IgnoreSelf?` TraceColor TraceHitColor DrawTime))
      (if _returnvalue_4
        (return true _outhit_2)
        (else
          (return false (`GameplayStatics.MakeHitResult` false false 0.0 0.0 (0.0 0.0 0.0) (0.0 0.0 0.0) (0.0 0.0 1.0) (0.0 0.0 1.0) null null null "None" 0 0 _returnvalue _returnvalue_2)))))))

(fn `AGR_RegenFloat`
  (params (Value :type "Float (double-precision) (by ref)") (PerSecond :type "Float (double-precision) (by ref)") (MIn :type "Float (double-precision) (by ref)") (Max :type "Float (double-precision) (by ref)"))
  (`|VariableSetRef` Value (`KismetMathLibrary.FClamp` (+ Value (* PerSecond (`GameplayStatics.GetWorldDeltaSeconds` null))) MIn Max)))

(fn `AGR_SphereTrace`
  (params (Origin :type "Actor Object Reference (by ref)") (SphereRadius :type "Float (double-precision)" :default 1000.0) (ObjectTypes :type "Array of EObjectTypeQuery Enum (by ref)") (ActorsToIgnore :type "Array of Actor Object Reference (by ref)") (ActorClassFilter :type "Object Class Reference"))
  (returns (ReturnValue :type Boolean) (OutActors :type "Array of Actor Object Reference"))
  (bind (_outactors _returnvalue) (`KismetSystemLibrary.SphereOverlapActors` Origin (`Actor.K2_GetActorLocation` Origin) SphereRadius ObjectTypes ActorClassFilter ActorsToIgnore))
  (return _returnvalue _outactors))