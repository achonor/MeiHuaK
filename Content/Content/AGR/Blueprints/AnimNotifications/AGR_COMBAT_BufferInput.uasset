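; Anim notify state that marks the combat input buffering window within an animation.
; On begin, it finds the owner's AGR_CombatMaster component and sets AllowsInput to true.
; On end, it closes input, sets AttackUnlocked and calls TryConsumeInput on that component, presumably so a buffered attack can fire.
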(fn `Received_NotifyBegin`
  (params (MeshComp :type "SkeletalMeshComponent Object Reference") (Animation :type "AnimSequenceBase Object Reference") (TotalDuration :type "Float (double-precision)"))
  (returns (ReturnValue :type Boolean))
  (bind _returnvalue (`Actor.GetComponentByClass` (`ActorComponent.GetOwner` MeshComp) "/Game/Content/AGR/Blueprints/AGR_CombatMaster.AGR_CombatMaster_C"))
  (`/Engine/EditorBlueprintResources/StandardMacros.IsValid` _returnvalue
    (:`Is Valid`
      (set `/Game/Content/AGR/Blueprints/AGR_CombatMaster.AllowsInput?` true _returnvalue)
      (return true))
    (:`Is Not Valid`
      (return false))))

(fn `Received_NotifyEnd`
  (params (MeshComp :type "SkeletalMeshComponent Object Reference") (Animation :type "AnimSequenceBase Object Reference"))
  (returns (ReturnValue :type Boolean))
  (bind _returnvalue (`Actor.GetComponentByClass` (`ActorComponent.GetOwner` MeshComp) "/Game/Content/AGR/Blueprints/AGR_CombatMaster.AGR_CombatMaster_C"))
  (`/Engine/EditorBlueprintResources/StandardMacros.IsValid` _returnvalue
    (:`Is Valid`
      (set `/Game/Content/AGR/Blueprints/AGR_CombatMaster.AllowsInput?` false _returnvalue)
      (set `/Game/Content/AGR/Blueprints/AGR_CombatMaster.AttackUnlocked?` true _returnvalue)
      (`/Game/Content/AGR/Blueprints/AGR_CombatMaster.TryConsumeInput` _returnvalue)
      (return false))
    (:`Is Not Valid`
      (return false))))