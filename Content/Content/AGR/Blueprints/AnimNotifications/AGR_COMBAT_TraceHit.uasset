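; Anim notify state that marks the window in an animation during which melee combat hit tracing is active.
; On begin it finds the AGR_CombatMaster component on the mesh owner and calls BeginCollisionTest; on end it calls FinishCollisionTest.
; If the component is missing, it prints an error message instead.
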(fn `Received_NotifyBegin`
  (params (MeshComp :type "SkeletalMeshComponent Object Reference") (Animation :type "AnimSequenceBase Object Reference") (TotalDuration :type "Float (double-precision)"))
  (returns (ReturnValue :type Boolean))
  (bind _returnvalue (`Actor.GetComponentByClass` (`ActorComponent.GetOwner` MeshComp) "/Game/Content/AGR/Blueprints/AGR_CombatMaster.AGR_CombatMaster_C"))
  (`/Engine/EditorBlueprintResources/StandardMacros.IsValid` _returnvalue
    (:`Is Valid`
      (`/Game/Content/AGR/Blueprints/AGR_CombatMaster.BeginCollisionTest` _returnvalue)
      (return true))
    (:`Is Not Valid`
      (`KismetSystemLibrary.PrintString` null "Notify Combat Trace error - no combat master component!")
      (return true))))

(fn `Received_NotifyEnd`
  (params (MeshComp :type "SkeletalMeshComponent Object Reference") (Animation :type "AnimSequenceBase Object Reference"))
  (returns (ReturnValue :type Boolean))
  (bind _returnvalue (`Actor.GetComponentByClass` (`ActorComponent.GetOwner` MeshComp) "/Game/Content/AGR/Blueprints/AGR_CombatMaster.AGR_CombatMaster_C"))
  (`/Engine/EditorBlueprintResources/StandardMacros.IsValid` _returnvalue
    (:`Is Valid`
      (`/Game/Content/AGR/Blueprints/AGR_CombatMaster.FinishCollisionTest` _returnvalue)
      (return true))
    (:`Is Not Valid`
      (`KismetSystemLibrary.PrintString` null "Notify Combat Trace error - no combat master component!")
      (return false))))