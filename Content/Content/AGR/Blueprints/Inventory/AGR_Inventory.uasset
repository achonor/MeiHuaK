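; AGR inventory component that lets its owning actor pick up and hold actors carrying an AGR_Item component, identified by a server-generated GUID.
; Stored items stay real actors, hidden without collision and attached to a character's PlayerState or the owner, with the GUID stamped on them.
; Item queries match that GUID among attached or tagged actors.
; Stackable pickups fill existing stacks, spawn actors for overflow, then destroy the original.
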(event `InitInventory`
  ;[0.3125 0 1] init
  (if (`KismetSystemLibrary.IsServer`)
    (set `self.InventoryID` (`KismetGuidLibrary.NewGuid`))))

(event `self.ReceiveBeginPlay`
  ;[0.4531 0 1] begin play
  (`self.InitInventory`)
  ;;[0.5469 0 1] char owner reference
  (bind `_as角色` (cast `Character` (`self.GetOwner`)))
  (set `self.OwnerAsCharacter` `_as角色`))

(fn `AddStacks`
  (params (ItemClass :type "Actor Class Reference") (Stacks :type Integer))
  (returns (Success :type Boolean))
  (locals (StacksToAdd :type Integer) (FreeSpace :type Integer :default 0))
  (bind _returnvalue (`self.GetOwner`))
  (bind _stackstoadd (`local.StacksToAdd`))
  (bind _returnvalue_2 (> (`local.StacksToAdd`) 0))
  ;[0.7813 0 1] Stacks, all items filter by class
  (set `local.StacksToAdd` Stacks)
  (bind _actors (`self.GetAllItems`))
  (bind _filteredarray (`KismetArrayLibrary.FilterArray` _actors ItemClass))
  ;[0 1 0.8359] Increase stacks of stackable items in inventory
  (for _array_element _filteredarray
    (bind _returnvalue_3 (`Actor.GetComponentByClass` _array_element "/Game/Content/AGR/Blueprints/Inventory/AGR_Item.AGR_Item_C"))
    (bind _stacksnow (`/Game/Content/AGR/Blueprints/Inventory/AGR_Item.StacksNow` _returnvalue_3))
    (bind _output_get (set `local.FreeSpace` (- (`/Game/Content/AGR/Blueprints/Inventory/AGR_Item.MaxStack` _returnvalue_3) _stacksnow)))
    (if (>= _output_get (`local.StacksToAdd`))
      (set `/Game/Content/AGR/Blueprints/Inventory/AGR_Item.StacksNow` (+ _stacksnow (`local.StacksToAdd`)) _returnvalue_3)
      (set `local.StacksToAdd` 0)
      (else
        (set `/Game/Content/AGR/Blueprints/Inventory/AGR_Item.StacksNow` (`/Game/Content/AGR/Blueprints/Inventory/AGR_Item.MaxStack` _returnvalue_3) _returnvalue_3)
        (set `local.StacksToAdd` (- (`local.StacksToAdd`) (`local.FreeSpace`)))))
    (if (<= (`local.StacksToAdd`) 0)
      (break)))
  ;[0.4766 0 1] Creater new items with max stack until all StacksAdded
  (if _returnvalue_2
    (while _returnvalue_2
      (bind _returnvalue_4 (`|SpawnActorFromClass` ItemClass (`Actor.GetTransform` _returnvalue) "AlwaysSpawn" "OverrideRootScale" _returnvalue (`Actor.Instigator` _returnvalue)))
      (bind _returnvalue_5 (`Actor.GetComponentByClass` _returnvalue_4 "/Game/Content/AGR/Blueprints/Inventory/AGR_Item.AGR_Item_C"))
      (bind _maxstack (`/Game/Content/AGR/Blueprints/Inventory/AGR_Item.MaxStack` _returnvalue_5))
      (if (<= _stackstoadd _maxstack)
        (set `/Game/Content/AGR/Blueprints/Inventory/AGR_Item.StacksNow` _stackstoadd _returnvalue_5)
        (set `local.StacksToAdd` 0)
        (else
          (set `/Game/Content/AGR/Blueprints/Inventory/AGR_Item.StacksNow` _maxstack _returnvalue_5)
          (set `local.StacksToAdd` (- _stackstoadd _maxstack))))
      ;[0 1 0.7188] register in inventory directly
      (`self.RawAddToInventory` _returnvalue_4)
      (`self.RawUpdateInventoryRef` _returnvalue_4)))
  ;[0 1 0.9531] finish
  (return true))

(fn `GetAllItems`
  (returns (Actors :type "Array of Actor Object Reference"))
  (locals (Inventory :type "Array of Actor Object Reference"))
  (bind _ownerascharacter (`self.OwnerAsCharacter`))
  ;[0.2422 1 0] start
  (`/Engine/EditorBlueprintResources/StandardMacros.IsValid` _ownerascharacter
    (:`Is Valid`
      ;[1 0.1172 0] player
      (for _array_element (`Actor.GetAttachedActors` (`Pawn.PlayerState` _ownerascharacter) true)
        (bind _returnvalue (`Actor.GetComponentByClass` _array_element "/Game/Content/AGR/Blueprints/Inventory/AGR_Item.AGR_Item_C"))
        (`/Engine/EditorBlueprintResources/StandardMacros.IsValid` _returnvalue
          (:`Is Valid`
            (if (== (`/Game/Content/AGR/Blueprints/Inventory/AGR_Item.InventoryID` _returnvalue) (`self.InventoryID`))
              (`KismetArrayLibrary.Array_Add` (`local.Inventory`) _array_element))))))
    (:`Is Not Valid`
      ;[1 0 0.7969] non character
      (bind _outactors (`GameplayStatics.GetAllActorsOfClassWithTag` "/Script/Engine.Actor" "AGR_ITEM"))
      (for _array_element_2 _outactors
        (bind _returnvalue_2 (`Actor.GetComponentByClass` _array_element_2 "/Game/Content/AGR/Blueprints/Inventory/AGR_Item.AGR_Item_C"))
        (`/Engine/EditorBlueprintResources/StandardMacros.IsValid` _returnvalue_2
          (:`Is Valid`
            (if (== (`/Game/Content/AGR/Blueprints/Inventory/AGR_Item.InventoryID` _returnvalue_2) (`self.InventoryID`))
              (`KismetArrayLibrary.Array_Add` (`local.Inventory`) _array_element_2)))))))
  ;[0.8984 0 1] return
  (return (`local.Inventory`)))

(fn `Guid as Name`
  (returns (ReturnValue :type Name))
  (return (`KismetStringLibrary.Conv_StringToName` (`KismetGuidLibrary.Conv_GuidToString` (`self.InventoryID`)))))

(fn `OnRep_InventoryID`
  (`KismetSystemLibrary.PrintText` (`|FormatText` "Inventory initialized: Owner {1}  - nventory ID {2}" (`KismetSystemLibrary.GetDisplayName` (`self.GetOwner`)) (`KismetGuidLibrary.Conv_GuidToString` (`self.InventoryID`))) (`self.Debug?`)))

(fn `RawAddToInventory`
  (params (Item :type "Actor Object Reference"))
  (`Actor.SetActorEnableCollision` Item false)
  (`Actor.SetActorHiddenInGame` Item true)
  (bind _ownerascharacter (`self.OwnerAsCharacter`)
    (:`then`
      (`Actor.K2_AttachToActor` Item (`Pawn.PlayerState` _ownerascharacter) "None" "SnapToTarget" "SnapToTarget" "KeepRelative" false))
    (:`else`
      (`Actor.K2_AttachToActor` Item (`self.GetOwner`) "None" "SnapToTarget" "SnapToTarget" "KeepRelative" false)))
  (return))

(fn `RawUpdateInventoryRef`
  (params (Item :type "Actor Object Reference"))
  (returns (Success :type Boolean))
  (bind _returnvalue (`Actor.GetComponentByClass` Item "/Game/Content/AGR/Blueprints/Inventory/AGR_Item.AGR_Item_C"))
  (`KismetArrayLibrary.Array_Add` (`Actor.Tags` Item) (`self.Guid as Name`))
  (`/Engine/EditorBlueprintResources/StandardMacros.IsValid` _returnvalue
    (:`Is Valid`
      (set `/Game/Content/AGR/Blueprints/Inventory/AGR_Item.InventoryID` (`self.InventoryID`) _returnvalue)
      (return true))
    (:`Is Not Valid`
      (return false))))

(fn `RawUpdateOwnership`
  (params (Item :type "Actor Object Reference"))
  (returns (Success :type Boolean))
  (bind _returnvalue (`Actor.GetComponentByClass` Item "/Game/Content/AGR/Blueprints/Inventory/AGR_Item.AGR_Item_C"))
  (bind _returnvalue_2 (`self.GetOwner`))
  (set `Actor.bNetUseOwnerRelevancy` true Item)
  (`/Engine/EditorBlueprintResources/StandardMacros.IsValid` _returnvalue
    (:`Is Valid`
      (`Actor.SetOwner` Item _returnvalue_2)
      (bind _ownerascharacter (`self.OwnerAsCharacter`)
        (:`then`
          (set `Actor.Instigator` _ownerascharacter Item))
        (:`else`
          (set `Actor.Instigator` (`Actor.Instigator` _returnvalue_2) Item)))
      (set `/Game/Content/AGR/Blueprints/Inventory/AGR_Item.OwnersID` (`self.InventoryID`) _returnvalue)
      (return true))
    (:`Is Not Valid`
      (return false))))

(fn `TryPickupItem`
  (params (PickupActor :type "Actor Object Reference"))
  (returns (Success :type Boolean))
  (locals (`Success?` :type Boolean :default false) (AttachSocket :type Name) (SuccessfullAttach :type Boolean) (Item :type "Actor Object Reference") (ItemComponent :type "/Game/Content/AGR/Blueprints/Inventory/AGR_Item Object Reference"))
  (bind _returnvalue (`Actor.GetComponentByClass` PickupActor "/Game/Content/AGR/Blueprints/Inventory/AGR_Item.AGR_Item_C"))
  ;[0.4531 0 1] can be picked up
  (bind _output_get (set `local.Success?` (`KismetSystemLibrary.IsValid` _returnvalue)))
  (if _output_get
    (bind _output_get_2 (set `local.ItemComponent` _returnvalue))
    (bind _output_get_3 (set `local.Item` PickupActor))
    ;[0.8516 1 0] stackable
    (if (`/Game/Content/AGR/Blueprints/Inventory/AGR_Item.Stackable?` _output_get_2)
      (bind _success (`self.AddStacks` (`GameplayStatics.GetObjectClass` _output_get_3) (`/Game/Content/AGR/Blueprints/Inventory/AGR_Item.StacksNow` _output_get_2)))
      (bind _output_get_4 (set `local.Success?` _success))
      (if _output_get_4
        (`Actor.K2_DestroyActor` _output_get_3)
        (return _output_get_4)
        (else
          (return _output_get_4)))
      (else
        ;[0.9219 0 1] raw add unique item
        (`self.RawAddToInventory` _output_get_3)
        (`self.RawUpdateInventoryRef` _output_get_3)
        (`self.RawUpdateOwnership` _output_get_3)
        (return true)))
    (else
      (return false))))