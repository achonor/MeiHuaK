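; AGR_Interface is a Blueprint Interface that declares the shared functions for communication between AGR Blueprints, with no logic of its own.
; Getters expose the look-at target, mouse target trace by channel, active camera, aim component and socket, alliance tags and hand IK positions.
; Setters toggle look-at-cursor, cursor visibility and debug mode, while InterfaceEventByName passes a generic named event to the implementer.
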(fn `GetActiveCamera`
  (returns (Camera :type "CameraComponent Object Reference"))
  (return null))

(fn `GetAimFromComponent`
  (returns (component :type "SceneComponent Object Reference") (`UseSocket?` :type Boolean) (SocketName :type Name))
  (return null false "None"))

(fn `GetAllianceTags`
  (returns (Friendly :type "Array of Name") (Enemy :type "Array of Name"))
  (return))

(fn `GetHandsIK`
  (returns (HandR :type "Vector Structure") (HandL :type "Vector Structure"))
  (return (0.0 0.0 0.0) (0.0 0.0 0.0)))

(fn `GetLookAtTarget`
  (returns (Target :type "Actor Object Reference"))
  (return null))

(fn `GetMouseTarget`
  (params (Channel :type "ETraceTypeQuery Enum" :default "TraceTypeQuery1") (`Complex?` :type Boolean))
  (returns (Success :type Boolean) (UnderMouseHit :type "HitResult Structure"))
  (return false))

(fn `InterfaceEventByName`
  (params (Name :type Name)))

(fn `SetDebugMode`
  (params (`GoIntoDebug?` :type Boolean)))

(fn `SetLookAtCursor`
  (params (LookAtCursor :type Boolean)))

(fn `SetShowCursor`
  (params (`ShowCursor?` :type Boolean)))