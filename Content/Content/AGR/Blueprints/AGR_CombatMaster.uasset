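; Melee combat component for a Character owner, handling combo attacks, weapon hit detection and target acquisition.
; Buffered input keys look up montages in a combo map, replicated via server and multicast, with a timer resetting the combo.
; Timed multi-line traces between previous and current socket positions on registered colliders report hits, filtered by ignore lists.
; Sphere queries pick the closest or best-angle aim target, also setting AI focus.
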(event `SetupDebug`
  (params (`Debug?` :type Boolean))
  ;[1 0.3984 0] SetupDebug
  (set `self.Debug?` `Debug?`))

(event `self.ReceiveBeginPlay`
  ;[0.1719 1 0] Begin Play - references
  (`self.GetOwnerAsCharRef`)
  (`KismetSystemLibrary.Delay` 0.2)
  (`self.GetOwnerAsCharRef`)
  (`self.SetAllAttacksToDefault`))

(event `SetupDefaultAttacks`
  (params (DefaultAttacks :type "Map of GameplayTag Structure to AnimMontage Object Reference"))
  ;[1 0.9609 0] Setup Default Attacks table
  (set `self.DefaultAttacks` DefaultAttacks))

(event `SetupAuthorityComboResetTime`
  (params (ComboAutoResetTimer :type "Float (double-precision)"))
  ;[0.4297 0 1] Setup Combo reset
  (`self.OwnerAuthority`
    (:`Authority`
      (set `self.ComboAutoResetTimer` ComboAutoResetTimer))
    (:`Remote`
      (`KismetSystemLibrary.PrintString` "Only server can change this value. It could be important for long attacks - best run by anim notification on server"))))

(event `SetupTryBufferInput`
  (params (InputBuffer :type "GameplayTag Structure"))
  ;[0 1 0.8828] Input Buffer
  (if (`self.AllowsInput?`)
    (bind _output_get (set `self.InputBuffer` InputBuffer))
    (`self.TryConsumeInput`)))

(event `PlayNetworkedMontage`
  (params (Montage :type "AnimMontage Object Reference") (PlayRate :type "Float (double-precision)" :default 1.0) (StartingSection :type Name) (Move :type "GameplayTag Structure"))
  ;[0 1 0.7422] Multiplayer Animation Montage
  (if (`self.LocalControlled`)
    (`|PlayMontage` (`Character.Mesh` (`self.CharacterOwnerRef`)) Montage PlayRate 0.0 StartingSection
      (:`then`
        (`self.BegunAttack` Move)
        (`self.ServerPlayMontage` Montage PlayRate StartingSection Move))
      (:`OnCompleted`
        (`self.EndedAttack` Move :!label _label))
      (:`OnInterrupted`
        (goto _label)))))

(event `SetupRegisterCollisionMesh`
  (params (RegisterByName :type Name) (Component :type "ActorComponent Object Reference"))
  (bind _savedcolliders (`self.SavedColliders`))
  ;[1 0 0.8203] Register Collider - good practice is to threat the "name" as "slot" in example "sword" or "right hand weapon"
  (`BlueprintMapLibrary.Map_Remove` _savedcolliders RegisterByName)
  (`BlueprintMapLibrary.Map_Add` _savedcolliders RegisterByName Component)
  (`self.ServerRegisterMesh` RegisterByName Component))

(event `TryConsumeInput`
  ;[1 0 0.9375] Consume Input Buffer
  (if (`self.AttackUnlocked?`)
    (`self.ExecuteAttack` (`self.InputBuffer`))
    ;;[0.8984 1 0] invalidate on consume
    (set `self.InputBuffer` (struct))))

(event `ServerPlayMontage`
  (params (MontageToPlay :type "AnimMontage Object Reference") (PlayRate :type "Float (double-precision)") (StartingSection :type Name) (NewParam :type "GameplayTag Structure"))
  ;[0 1 0.7422] Multiplayer Animation Montage
  (`/Engine/EditorBlueprintResources/StandardMacros.IsValid` (`self.CharacterOwnerRef`)
    (:`Is Valid`
      _)
    (:`Is Not Valid`
      (`self.GetOwnerAsCharRef`)))
  (`|PlayMontage` (`Character.Mesh` (`self.CharacterOwnerRef`)) MontageToPlay PlayRate 0.0 StartingSection
    (:`then`
      (`self.BegunAttack` NewParam)
      (`self.MultiPlayMontage` MontageToPlay PlayRate StartingSection NewParam))
    (:`OnCompleted`
      (`self.EndedAttack` NewParam :!label _label_2))
    (:`OnInterrupted`
      (goto _label_2))))

(event `ServerRegisterMesh`
  (params (Name :type Name) (Component :type "ActorComponent Object Reference (by ref)"))
  (bind _savedcolliders (`self.SavedColliders`))
  ;[1 0 0.8203] Register Collider - good practice is to threat the "name" as "slot" in example "sword" or "right hand weapon"
  (`BlueprintMapLibrary.Map_Remove` _savedcolliders Name)
  (`BlueprintMapLibrary.Map_Add` _savedcolliders Name Component))

(event `ExecuteAttack`
  (params (Key :type "GameplayTag Structure (by ref)"))
  (bind (_value _returnvalue) (`BlueprintMapLibrary.Map_Find` (`self.CurrentComboAttack`) Key))
  ;[1 0 0.9609] StartBuffered Attack
  (if (and _returnvalue (`self.AttackUnlocked?`))
    (`/Engine/EditorBlueprintResources/StandardMacros.IsValid` _value
      (:`Is Valid`
        (`self.PlayNetworkedMontage` _value 1.0 "None" Key)
        (set `self.AttackUnlocked?` false)
        ;[0 1 0.1094] FailSafe Reset Combo
        (bind _returnvalue_2 (`KismetSystemLibrary.K2_SetTimer` self "SetAllAttacksToDefault" (`self.ComboAutoResetTimer`)))
        (set `self.ResetTimerHandle` _returnvalue_2)))))

(event `SetupActivateCollider`
  (params (Key :type Name) (`ClearOthers?` :type Boolean))
  ;[0.7578 1 0] Setup active collider
  (`self.TryActivateCollider` Key `ClearOthers?`)
  (`self.ServerActivateCollider` Key `ClearOthers?`))

(event `MultiPlayMontage`
  (params (AnimMontage :type "AnimMontage Object Reference") (InPlayRate :type "Float (double-precision)") (StartSectionName :type Name) (Move :type "GameplayTag Structure"))
  ;[0 1 0.7422] Multiplayer Animation Montage
  (if (`KismetMathLibrary.BooleanNOR` (`KismetSystemLibrary.IsServer`) (`self.LocalControlled`))
    (`/Engine/EditorBlueprintResources/StandardMacros.IsValid` (`self.CharacterOwnerRef`)
      (:`Is Valid`
        _)
      (:`Is Not Valid`
        (`self.GetOwnerAsCharRef`)))
    (`|PlayMontage` (`Character.Mesh` (`self.CharacterOwnerRef`)) AnimMontage InPlayRate 0.0 StartSectionName
      (:`then`
        (`self.BegunAttack` Move))
      (:`OnCompleted`
        (`self.EndedAttack` Move :!label _label_3))
      (:`OnInterrupted`
        (goto _label_3)))))

(event `ServerActivateCollider`
  (params (ActiveName :type Name) (`ClearOthers?` :type Boolean))
  ;[0.7578 1 0] Setup active collider
  (`self.TryActivateCollider` ActiveName `ClearOthers?`))

(event `SetAllAttacksToDefault`
  ;[0.7344 0 1] Reset all attacks to default
  (set `self.CurrentComboAttack` (`self.DefaultAttacks`))
  (set `self.AllowsInput?` true)
  (set `self.AttackUnlocked?` true)
  (`self.ComboEnded`))

(event `SetupAuthorityCollisionPreset`
  (params (CollisionStartSocket :type Name :default "start") (CollisionEndSocket :type Name :default "stop") (MeleeCollisionPrecision :type Integer :default 10) (TracesPerSec :type "Float (double-precision)") (`ComplexCollision?` :type Boolean) (MeleeCollisionChannel :type "ETraceTypeQuery Enum" :default "TraceTypeQuery1") (`TraceOnlyOnServer?` :type Boolean))
  ;[0 1 0.03906] Setup Collision Presets
  (`self.OwnerAuthority`
    (:`Authority`
      (set `self.CollisionStartSocket` CollisionStartSocket)
      (set `self.CollisionEndSocket` CollisionEndSocket)
      (set `self.MeleeCollisionPrecision` MeleeCollisionPrecision)
      (set `self.TracesPerSec` TracesPerSec)
      (set `self.ComplexCollision?` `ComplexCollision?`)
      (set `self.MeleeCollisionChannel` MeleeCollisionChannel)
      (set `self.TraceOnlyOnServer?` `TraceOnlyOnServer?`))
    (:`Remote`
      (`KismetSystemLibrary.PrintString` "This Event Can be triggered only on the server! MEssing those settings could crash the server!"))))

(event `SetNextAttackInCombo`
  (params (Key :type "GameplayTag Structure") (Montage :type "AnimMontage Object Reference (by ref)"))
  (bind _currentcomboattack (`self.CurrentComboAttack`))
  ;[1 0 0.1172] Set Next combo
  (`BlueprintMapLibrary.Map_Remove` _currentcomboattack Key)
  (`BlueprintMapLibrary.Map_Add` _currentcomboattack Key Montage))

(event `SetupAuthorityAddToIgnoreList`
  (params (IgnoreActors :type "Array of Actor Object Reference") (IgnoreClasses :type "Array of Actor Class Reference"))
  ;[0 1 0.7891] Update Ignore List If Authority!
  (`self.OwnerAuthority`
    (:`Authority`
      (`KismetArrayLibrary.Array_Append` (`self.HitIgnoreClasses`) IgnoreClasses)
      (`KismetArrayLibrary.Array_Append` (`self.HitIgnoreActors`) IgnoreActors))
    (:`Remote`
      (`KismetSystemLibrary.PrintString` "This Event Can be triggered only on the server! MEssing those settings could allow cheating!"))))

(event `TryActivateCollider`
  (params (ActiveName :type Name) (`ClearOthers?` :type Boolean))
  (bind _activecolliders (`self.ActiveColliders`))
  (bind (_value _returnvalue) (`BlueprintMapLibrary.Map_Find` (`self.SavedColliders`) ActiveName))
  ;[0 0.9531 1] Try Activate Collider
  ;;[1 0 0.8437] Clear If set to do so
  (if `ClearOthers?`
    (`KismetArrayLibrary.Array_Clear` _activecolliders))
  ;;[0 0.01562 1] set active
  (if _returnvalue
    (`KismetArrayLibrary.Array_AddUnique` _activecolliders _value)
    (else
      (`KismetSystemLibrary.PrintString` "No such Collider Registered! Use \"SetupRegisterCollisionMesh\""))))

(event `SetupAuthorityRemoveFromIgnoreList`
  (params (Actors :type "Array of Actor Object Reference") (ActorClass :type "Array of Actor Class Reference"))
  ;[1 0.3281 0] Remove ignored actors
  (`|ExecutionSequence`
    (:`then_0`
      (for _array_element Actors
        (`KismetArrayLibrary.Array_RemoveItem` (`self.HitIgnoreActors`) _array_element)))
    (:`then_1`
      (for _array_element_2 ActorClass
        (`KismetArrayLibrary.Array_RemoveItem` (`self.HitIgnoreClasses`) _array_element_2)))))

(event `BeginCollisionTest`
  ;[0 1 0.25] Start and stop collision checks - minimum 2 frames. default 30/second (anim speed)
  ;;[0 1 1] Begin
  (`self.BegunHitTrace`)
  (bind _returnvalue (`KismetSystemLibrary.K2_SetTimerDelegate` (delegate `CollisionTestSingleFrame`) (/ 1.0 (`self.TracesPerSec`)) true))
  (set `self.CollisionTimer` _returnvalue)
  ;;[0 0.8359 1] BeforeFirst Attack - save last socket position per active collider
  (for (_array_element _array_index) (`self.ActiveColliders`)
    (bind `_as场景组件` (cast `SceneComponent` _array_element))
    (bind (_start _end) (`self.GetSockets` `_as场景组件`))
    (`KismetArrayLibrary.Array_Set` (`self.PrevFrameStart`) _array_index _start true)
    (`KismetArrayLibrary.Array_Set` (`self.PrevFrameStop`) _array_index _end true))
  ;;[1 0 0.04687] First frame Forced
  (`self.CollisionTestSingleFrame`))

(event `FinishCollisionTest`
  ;[0 1 0.25] Start and stop collision checks - minimum 2 frames. default 30/second (anim speed)
  ;;[1 0 0.5859] End
  (`KismetSystemLibrary.K2_ClearAndInvalidateTimerHandle` (`self.CollisionTimer`))
  (`self.CollisionTestSingleFrame`)
  (`self.EndedHitTrace`))

(event `CollisionTestSingleFrame`
  ;[0 1 0.5078] Collision test
  ;;[1 0.7031 0] Start collision check for each active collider
  (if (`self.TraceOnlyOnServer?`)
    (`self.OwnerAuthority`
      (:`Authority`
        _)))
  (for (_array_element _array_index) (`self.ActiveColliders`)
    (bind `_as场景组件` (cast `SceneComponent` _array_element)
      (:`then`
        ;;[0.03035 1 0.9602] Per Point collision with N precision
        (for _index (range (+ (`self.MeleeCollisionPrecision`) 1))
          (bind (_start _stop) (`self.GetPrevFrameSockets` _array_index))
          (bind (_start_2 _end) (`self.GetSockets` `_as场景组件`))
          (bind (_outhits _returnvalue) (`KismetSystemLibrary.LineTraceMulti` (`self.CalculateTracePoint` _index _start _stop) (`self.CalculateTracePoint` _index _start_2 _end) (`self.MeleeCollisionChannel`) (`self.ComplexCollision?`) (`self.HitIgnoreActors`) (select `bool` (`self.Debug?`) :`true` "ForDuration" :!type "EDrawDebugTrace Enum") true (struct :`G` 0.409151 :`B` 0.4375 :`A` 1.0) (struct :`R` 0.977619 :`G` 1.0 :`A` 1.0) 0.1))
          ;;;[1 0 0.6562] For each hit
          (if _returnvalue
            (for _array_element_2 _outhits
              ;;[1 0.3516 0] Check Ignore Lists
              (if (not (`KismetArrayLibrary.Array_Contains` (`self.HitIgnoreClasses`) (`GameplayStatics.GetObjectClass` (`.HitActor` (`GameplayStatics.BreakHitResult` _array_element_2)))))
                ;;[0.1719 0 1] Call EventDispatcherHit
                (`self.HandleRegisteredHit` _array_element_2)))))
        ;;;[0.007812 1 0] Save Previous Frame
        (`KismetArrayLibrary.Array_Set` (`self.PrevFrameStart`) _array_index _start_2 true)
        (`KismetArrayLibrary.Array_Set` (`self.PrevFrameStop`) _array_index _end true))
      (:`CastFailed`
        ;;[0 0.2266 1] Cant Trace?
        (`KismetSystemLibrary.PrintString` "ColliderComponent is not a scene component - therefore cant handle sockets!")))))

(event `SetupAimAssist`
  (params (`Autoaim?` :type Boolean) (AutoaimSpeed :type "Float (double-precision)"))
  ;[1 0.04688 0] Auto aim
  (set `self.Autoaim?` `Autoaim?`)
  (set `self.AutoaimSpeed` AutoaimSpeed))

(event `SetupAimTarget`
  (params (AimTarget :type "Actor Object Reference"))
  (bind _characterownerref (`self.CharacterOwnerRef`))
  ;[0 1 0.6719] Aim Target
  (bind _output_get (set `self.AimTarget` AimTarget))
  ;;[0 1 0.9063] Ai focus target
  (if (not (`Pawn.IsPlayerControlled` _characterownerref))
    (`AIController.K2_SetFocus` (`AIBlueprintHelperLibrary.GetAIController` _characterownerref) _output_get)))

(event `ClearAimTarget`
  (bind _characterownerref (`self.CharacterOwnerRef`))
  ;[0 1 0.6719] Aim Target
  (set `self.AimTarget` null)
  ;;[0 1 0.9063] Ai focus target
  (if (not (`Pawn.IsPlayerControlled` _characterownerref))
    (`AIController.K2_SetFocus` (`AIBlueprintHelperLibrary.GetAIController` _characterownerref) null)))

(event `AimQueryForTargets`
  (params (Range :type "Float (double-precision)" :default 1500.0) (AcceptableAngle :type "Float (double-precision)" :default 90.0) (`TargetClosest?` :type Boolean) (`FromCamera?` :type Boolean :default true) (OnlyNewTarget :type Boolean) (ObjectTypes :type "Array of EObjectTypeQuery Enum (by ref)"))
  (bind _returnvalue (`GameplayStatics.GetPlayerCameraManager` 0))
  (bind _characterownerref (`self.CharacterOwnerRef`))
  (bind _debug_ (`self.Debug?`))
  ;[1 0.2344 0] Find Targets
  ;;[1 0 0.3281] Start
  ;;[0.4297 0 1] Debug
  (if (`self.Debug?`)
    (`KismetSystemLibrary.DrawDebugSphere` (select `bool` `FromCamera?` :`false` (`Actor.K2_GetActorLocation` _characterownerref) :`true` (`SceneComponent.K2_GetComponentLocation` (`PlayerCameraManager.TransformComponent` _returnvalue))) Range 48 (struct :`R` 1.0 :`G` 1.0 :`B` 1.0 :`A` 1.0) 1.0 3.0))
  ;;[1 0 0.3281] Sphere hit trace
  ;;;[0 1 0.1094] no target
  (bind (_returnvalue_2 _outactors) (`/Game/Content/AGR/Blueprints/AGR_LIBRARY.AGR_SphereTrace` (select `bool` `FromCamera?` :`false` _characterownerref :`true` _returnvalue :!type "Actor Object Reference") Range ObjectTypes (`self.HitIgnoreActors`)))
  (if _returnvalue_2
    (set `self.LastQueryTargets` _outactors)
    ;;;;[1 0.9844 0] New target check
    (if OnlyNewTarget
      (`KismetArrayLibrary.Array_RemoveItem` (`self.LastQueryTargets`) (`self.AimTarget`)))
    ;;[0 1 0.9766] Closest target
    (if `TargetClosest?`
      (bind (_target _distance) (`/Game/Content/AGR/Blueprints/AGR_LIBRARY.AGR_BestClosestTarget` _characterownerref (`self.LastQueryTargets`)))
      (bind _returnvalue_3 (`Actor.GetDotProductTo` (select `bool` `FromCamera?` :`false` _characterownerref :`true` _returnvalue :!type "Actor Object Reference") _target))
      ;;;[0.9453 1 0] Dot product check
      (if (> _returnvalue_3 (`KismetMathLibrary.MapRangeClamped` (`KismetMathLibrary.Abs` AcceptableAngle) 0.0 180.0 1.0 -1.0))
        (`self.SetupAimTarget` _target)
        ;;[0.1953 1 0] Debug draw
        (`KismetSystemLibrary.PrintString` (`KismetStringLibrary.Conv_DoubleToString` _returnvalue_3) _debug_)
        (`KismetSystemLibrary.PrintString` (`KismetStringLibrary.Conv_DoubleToString` _distance) _debug_)
        (if _debug_ :!label _label
          (`KismetSystemLibrary.DrawDebugSphere` (`Actor.K2_GetActorLocation` (`self.AimTarget`)) 100.0 12 (struct :`G` 0.435294 :`B` 0.007843 :`A` 1.0) 2.0 2.0))
        (else
          ;;;[0 0.08594 1] invalidate target
          (`self.ClearAimTarget`)))
      (else
        ;;[0 1 0.9531] Best Dot product target
        (bind (_besttarget _bestdot) (`/Game/Content/AGR/Blueprints/AGR_LIBRARY.AGR_BestDotTarget` (select `bool` `FromCamera?` :`false` _characterownerref :`true` _returnvalue :!type "Actor Object Reference") (`self.LastQueryTargets`)))
        ;;;[0.1719 0 1] Dot product check
        (if (> _bestdot (`KismetMathLibrary.MapRangeClamped` (`KismetMathLibrary.Abs` AcceptableAngle) 0.0 180.0 1.0 -1.0))
          (`self.SetupAimTarget` _besttarget)
          (`KismetSystemLibrary.PrintString` (`KismetStringLibrary.Conv_DoubleToString` _bestdot) _debug_)
          (goto _label)
          (else
            ;;;[0 1 0.6016] invalidate target
            (`self.ClearAimTarget`)))))
    (else
      (`self.ClearAimTarget`))))

(fn `CalculateTracePoint`
  (params (CurrentPoint :type Integer) (Start :type "Vector Structure") (End :type "Vector Structure"))
  (returns (ReturnValue :type "Vector Structure"))
  (return (+ Start (* (/ (- End Start) (`self.MeleeCollisionPrecision`)) CurrentPoint))))

(fn `GetAutoaimTarget?`
  (returns (ActiveAndValid :type Boolean) (AimTarget :type "Actor Object Reference"))
  (bind _aimtarget (`self.AimTarget`))
  (return (and (`self.Autoaim?`) (`KismetSystemLibrary.IsValid` _aimtarget)) _aimtarget))

(fn `GetOwnerAsCharRef`
  (returns (Reference :type "Character Object Reference"))
  (bind _returnvalue (`self.GetOwner`))
  (bind `_as角色` (cast `Character` (`self.GetOwner`))
    (:`then`
      (bind _output_get (set `self.CharacterOwnerRef` `_as角色`))
      (return _output_get))
    (:`CastFailed`
      (`KismetSystemLibrary.PrintString` (`KismetStringLibrary.Concat_StrStr` "Fatal error! CombatComponent has no owner character!" "   Object: " (`KismetSystemLibrary.GetObjectName` _returnvalue) "     display: " (`KismetSystemLibrary.GetDisplayName` _returnvalue)))
      (return null))))

(fn `GetPrevFrameSockets`
  (params (Index :type Integer))
  (returns (Start :type "Vector Structure (by ref)") (Stop :type "Vector Structure (by ref)"))
  (return (`|GetArrayItem` (`self.PrevFrameStart`) Index) (`|GetArrayItem` (`self.PrevFrameStop`) Index)))

(fn `GetSockets`
  (params (Component :type "SceneComponent Object Reference"))
  (returns (Start :type "Vector Structure") (End :type "Vector Structure"))
  (return (`SceneComponent.GetSocketLocation` Component (`self.CollisionStartSocket`)) (`SceneComponent.GetSocketLocation` Component (`self.CollisionEndSocket`))))

(fn `HasInputBuffer?`
  (returns (`ValidInputBuffered?` :type Boolean))
  (return (`BlueprintGameplayTagLibrary.IsGameplayTagValid` (`self.InputBuffer`))))

(fn `IsDefaultAttack`
  (params (Key :type "GameplayTag Structure (by ref)"))
  (returns (ReturnValue :type Boolean))
  (bind (_value _returnvalue) (`BlueprintMapLibrary.Map_Find` (`self.CurrentComboAttack`) Key))
  (bind (_value_2 _returnvalue_2) (`BlueprintMapLibrary.Map_Find` (`self.DefaultAttacks`) Key))
  (return (and _returnvalue_2 (== _value _value_2) _returnvalue)))

(fn `LocalControlled`
  (returns (ReturnValue :type Boolean))
  (bind _returnvalue (`Pawn.GetController` (`self.CharacterOwnerRef`)))
  (`/Engine/EditorBlueprintResources/StandardMacros.IsValid` (`self.CharacterOwnerRef`)
    (:`Is Valid`
      (`/Engine/EditorBlueprintResources/StandardMacros.IsValid` _returnvalue
        (:`Is Valid`
          _)))
    (:`Is Not Valid`
      (`self.GetOwnerAsCharRef`)))
  (return (`Controller.IsLocalController` _returnvalue)))