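; AGR player controller that handles cursor-driven look, autoaim rotation and cursor locking for the possessed pawn.
; It caches the pawn's AGR animation, combat and sound components, clears them on unpossess, and forwards debug mode to them.
; Each tick optionally faces the traced cursor hit, interpolates control rotation from the pawn's aim origin toward the autoaim target, and can pin the hidden cursor in place.
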(event `self.ReceiveBeginPlay`
  (bind _returnvalue (`self.K2_GetPawn`))
  ;[0 0.6719 1] Begin play
  (`KismetSystemLibrary.Delay` 0.0)
  (`/Engine/EditorBlueprintResources/StandardMacros.IsValid` _returnvalue
    (:`Is Valid`
      (`self.EventGetAGRReferences` _returnvalue))))

(event `self.ReceivePossess`
  (params (PossessedPawn :type "Pawn Object Reference"))
  ;[0 0.2031 1] Character possess
  (`self.EventGetAGRReferences` PossessedPawn))

(event `self.ReceiveUnPossess`
  (params (UnpossessedPawn :type "Pawn Object Reference"))
  ;[0 0.2031 1] Character possess
  ;;[1 0 0] Invalidate components
  (set `self.AnimationComponent` null)
  (set `self.CombatComponent` null)
  (set `self.SoundComponent` null))

(event `EventGetAGRReferences`
  (params (Target :type "Actor Object Reference"))
  (bind _returnvalue (`self.GetComponentByClass` Target "/Game/Content/AGR/Blueprints/AGR_SoundMaster.AGR_SoundMaster_C"))
  (bind _returnvalue_2 (`self.GetComponentByClass` Target "/Game/Content/AGR/Blueprints/AGR_AnimationMaster.AGR_AnimationMaster_C"))
  (bind _returnvalue_3 (`self.GetComponentByClass` Target "/Game/Content/AGR/Blueprints/AGR_CombatMaster.AGR_CombatMaster_C"))
  ;[0.03125 1 0] Agr components references
  (`|ExecutionSequence`
    (:`then_0`
      (`/Engine/EditorBlueprintResources/StandardMacros.IsValid` _returnvalue_2
        (:`Is Valid`
          (set `self.AnimationComponent` _returnvalue_2))))
    (:`then_1`
      (`/Engine/EditorBlueprintResources/StandardMacros.IsValid` _returnvalue_3
        (:`Is Valid`
          (set `self.CombatComponent` _returnvalue_3))))
    (:`then_2`
      (`/Engine/EditorBlueprintResources/StandardMacros.IsValid` _returnvalue
        (:`Is Valid`
          (set `self.SoundComponent` _returnvalue))))))

(event `EventSetRotation`
  (params (Start :type "Vector Structure (by ref)"))
  (bind _combatcomponent (`self.CombatComponent`))
  (bind (_activeandvalid _aimtarget) (`/Game/Content/AGR/Blueprints/AGR_CombatMaster.GetAutoaimTarget?` _combatcomponent))
  ;[1 0.01812 0.6912] Set rotation
  (if _activeandvalid
    (`self.SetControlRotation` (`KismetMathLibrary.RInterpTo` (`self.GetControlRotation`) (`KismetMathLibrary.FindLookAtRotation` Start (`self.GetActorEyesViewPoint` _aimtarget)) (`/Game/Content/AGR/Blueprints/AGR_CombatMaster.AutoaimSpeed` _combatcomponent) (`self.DeltaTimeX`)))))

(event `RunLookatCursor`
  ;[0.05157 0.3873 1] Look at cursor
  (if (`self.LookAtCursor`)
    (bind (_success _undermousehit) (`self.GetMouseTarget` "TraceTypeQuery1" true))
    (if _success
      (bind (_bblockinghit _binitialoverlap _time _distance _location) (`GameplayStatics.BreakHitResult` _undermousehit))
      (`self.SetControlRotation` (`KismetMathLibrary.FindLookAtRotation` (`self.K2_GetActorLocation` (`self.K2_GetPawn`)) _location))
      (if (`self.Debug`)
        (`KismetSystemLibrary.DrawDebugSphere` _location 20.0 12 (struct :`R` 0.002069 :`G` 0.604167 :`B` 0.190867 :`A` 1.0) 0.0 2.0)))))

(event `self.ReceiveTick`
  (params (DeltaSeconds :type "Float (single-precision)"))
  (bind (_locationx _locationy) (`self.GetMousePosition`))
  (bind (_mouseposition_x _mouseposition_y) (`KismetMathLibrary.BreakVector2D` (`self.MousePosition`)))
  ;[1 0 0.5391] Tick
  (set `self.DeltaTimeX` DeltaSeconds)
  (`|ExecutionSequence`
    (:`then_0`
      (`self.RunLookatCursor`))
    (:`then_1`
      (`self.RunAimAssistTick`))
    (:`then_2`
      (if (`self.LockCursorWhenNotVisible?`)
        (if (`self.bShowMouseCursor`)
          (goto _label :!via `Reset`)
          (else
            (`|ExecutionSequence`
              (:`then_0`
                (`/Engine/EditorBlueprintResources/StandardMacros.DoOnce` false :!label _label
                  (:`Completed`
                    (set `self.MousePosition` (`KismetMathLibrary.MakeVector2D` _locationx _locationy)))))
              (:`then_1`
                (`self.SetMouseLocation` (`KismetMathLibrary.FTrunc` _mouseposition_x) (`KismetMathLibrary.FTrunc` _mouseposition_y))))))))))

(event `RunAimAssistTick`
  (bind _returnvalue (`self.K2_GetPawn`))
  ;[1 0.4922 0] Aim Assist
  (if (`.combat` (`self.HasValidComponents?`))
    (if (`/Game/Content/AGR/Blueprints/AGR_CombatMaster.GetAutoaimTarget?` (`self.CombatComponent`))
      (`/Engine/EditorBlueprintResources/StandardMacros.IsValid` _returnvalue
        (:`Is Valid`
          (bind (_component _usesocket_ _socketname) (message `/Game/Content/AGR/Blueprints/AGR_Interface.GetAimFromComponent` _returnvalue))
          (`/Engine/EditorBlueprintResources/StandardMacros.IsValid` _component
            (:`Is Valid`
              (if _usesocket_
                (`self.EventSetRotation` (`SceneComponent.GetSocketLocation` _component _socketname))
                (else
                  (`self.EventSetRotation` (`SceneComponent.K2_GetComponentLocation` _component)))))
            (:`Is Not Valid`
              (`self.EventSetRotation` (`self.K2_GetActorLocation` _returnvalue)))))))))

(event `self.SetLookAtCursor`
  (params (LookAtCursor :type Boolean))
  ;[0.8516 1 0] AGR interface events
  (set `self.LookAtCursor` LookAtCursor))

(event `self.SetShowCursor`
  (params (`ShowCursor?` :type Boolean))
  ;[0.8516 1 0] AGR interface events
  (set `self.bShowMouseCursor` `ShowCursor?`))

(event `self.SetDebugMode`
  (params (`GoIntoDebug?` :type Boolean))
  (bind (_animation _combat _sound) (`self.HasValidComponents?`))
  ;[1 0 0.4687] Debug all components
  (`|ExecutionSequence`
    (:`then_0`
      (if _animation
        (set `/Game/Content/AGR/Blueprints/AGR_AnimationMaster.Debug?` `GoIntoDebug?` (`self.AnimationComponent`))))
    (:`then_1`
      (if _combat
        (`/Game/Content/AGR/Blueprints/AGR_CombatMaster.SetupDebug` (`self.CombatComponent`) `GoIntoDebug?`)))
    (:`then_2`
      (if _sound
        (set `/Game/Content/AGR/Blueprints/AGR_SoundMaster.Debug?` `GoIntoDebug?` (`self.SoundComponent`))))))

(fn `GetActiveCamera`
  (returns (Camera :type "CameraComponent Object Reference"))
  (return null))

(fn `GetAimFromComponent`
  (returns (component :type "SceneComponent Object Reference") (`UseSocket?` :type Boolean) (SocketName :type Name))
  (return null false "None"))

(fn `GetAllianceTags`
  (returns (Friendly :type "Array of Name") (Enemy :type "Array of Name"))
  (return))

(fn `GetHandsIK`
  (returns (HandR :type "Vector Structure") (HandL :type "Vector Structure"))
  (return (0.0 0.0 0.0) (0.0 0.0 0.0)))

(fn `GetLookAtTarget`
  (returns (Target :type "Actor Object Reference"))
  (return null))

(fn `GetMouseTarget`
  (params (Channel :type "ETraceTypeQuery Enum" :default "TraceTypeQuery1") (`Complex?` :type Boolean))
  (returns (Success :type Boolean) (UnderMouseHit :type "HitResult Structure"))
  (bind (_hitresult _returnvalue) (`self.GetHitResultUnderCursorByChannel` Channel `Complex?`))
  (if _returnvalue
    (return true _hitresult)
    (else
      (return false))))

(fn `HasValidComponents?`
  (returns (Animation :type Boolean) (combat :type Boolean) (Sound :type Boolean))
  (return (`KismetSystemLibrary.IsValid` (`self.AnimationComponent`)) (`KismetSystemLibrary.IsValid` (`self.CombatComponent`)) (`KismetSystemLibrary.IsValid` (`self.SoundComponent`))))

(fn `UserConstructionScript`)